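; Temple interior wall Blueprint that animates the opacity parameter of its child static meshes whenever its Opacity event is called.
; The construction script gathers those meshes and gives every material slot a dynamic material instance.
; Opacity plays one timeline on the "%OP" parameter once, while a retriggerable delay waits for calls to stop.
; After that delay, the DoOnce resets and a second timeline drives the same parameter.
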(event `Opacity`
  (`KismetSystemLibrary.PrintString` (`KismetStringLibrary.Conv_IntToString` (`KismetArrayLibrary.Array_Length` (`self.StaticMeshes`))))
  (`|ExecutionSequence`
    (:`then_0`
      (`/Engine/EditorBlueprintResources/StandardMacros.DoOnce` false :!label _label
        (:`Completed`
          (bind (_direction _newtrack_0) (`Timeline|Timeline_0` :!via `PlayFromStart`)
            (:`Update`
              (for _array_element (`self.DyamicMaterials`)
                (`MaterialInstanceDynamic.SetScalarParameterValue` _array_element "%OP" _newtrack_0)))))))
    (:`then_1`
      (`KismetSystemLibrary.RetriggerableDelay` 1.0)
      (`|ExecutionSequence`
        (:`then_0`
          (goto _label :!via `Reset`))
        (:`then_1`
          (bind (_direction_2 _newtrack_0_2) (`Timeline|Timeline_1` :!via `PlayFromStart`)
            (:`Update`
              (for _array_element_2 (`self.DyamicMaterials`)
                (`MaterialInstanceDynamic.SetScalarParameterValue` _array_element_2 "%OP" _newtrack_0_2)))))))))

(fn `SetMaterials`
  (params (StaticMeshes :type "StaticMeshComponent Object Reference (by ref)"))
  (for (_array_element _array_index) (`MeshComponent.GetMaterials` StaticMeshes)
    (bind _returnvalue (`PrimitiveComponent.CreateDynamicMaterialInstance` StaticMeshes _array_index _array_element "None"))
    (`PrimitiveComponent.SetMaterial` StaticMeshes _array_index _returnvalue)
    (`KismetArrayLibrary.Array_Add` (`self.DyamicMaterials`) _returnvalue)))

(fn `UserConstructionScript`
  (`KismetArrayLibrary.Array_Clear` (`self.DyamicMaterials`))
  (`KismetArrayLibrary.Array_Clear` (`self.StaticMeshes`))
  (for _array_element (`SceneComponent.GetChildrenComponents` (`self.DefaultSceneRoot`) true)
    (bind _asstatic_mesh_component (cast `StaticMeshComponent` _array_element))
    (`KismetArrayLibrary.Array_Add` (`self.StaticMeshes`) _asstatic_mesh_component))
  (for _array_element_2 (`self.StaticMeshes`)
    (`self.SetMaterials` _array_element_2)))