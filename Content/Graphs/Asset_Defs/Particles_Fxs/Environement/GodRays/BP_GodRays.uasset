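; BP_GodRays is an environment effect actor that pairs a god ray mesh with a spot light and a point light.
; All setup runs in the construction script, which aligns the anchor's pitch and yaw to a referenced directional light, with adjustable roll.
; Exposed variables drive mesh choice and XY scale, light properties and the spot light's light function material.
; Spot light color can optionally be copied from the directional light.
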(fn `UserConstructionScript`
  (bind _scalegodrays (`self.ScaleGodRays`))
  (bind (_returnvalue_roll _returnvalue_pitch _returnvalue_yaw) (`KismetMathLibrary.BreakRotator` (`self.K2_GetActorRotation` (`self.Directional_Light`))))
  (`SceneComponent.K2_SetWorldRotation` (`self.Anchor_Godray`) (`KismetMathLibrary.MakeRotator` (`self.GodRaysRotation`) _returnvalue_pitch _returnvalue_yaw) false false)
  (`StaticMeshComponent.SetStaticMesh` (`self.GodRays_Mesh`) (`self.Mesh_GD`))
  (if (`self.ColorSpotlight_Auto`)
    (set `self.ColorSpotLight_Bool` (`LightComponentBase.GetLightColor` (`Light.LightComponent` (`self.Directional_Light`))))
    (else
      (set `self.ColorSpotLight_Bool` (`self.ColorSpotLight`))))
  (`LightComponent.SetLightColor` (`self.SpotLight`) (`self.ColorSpotLight_Bool`) true)
  (`LightComponent.SetIntensity` (`self.SpotLight`) (`self.IntensitySpotLight`))
  (`SpotLightComponent.SetOuterConeAngle` (`self.SpotLight`) (`self.OuterConeAngle`))
  (`LightComponent.SetLightFunctionMaterial` (`self.SpotLight`) (`self.LightFunction`))
  (`SceneComponent.SetRelativeScale3D` (`self.GodRays_Mesh`) (`KismetMathLibrary.MakeVector` _scalegodrays _scalegodrays 1.0))
  (`SceneComponent.K2_SetRelativeRotation` (`self.SpotLight`) (`KismetMathLibrary.MakeRotator` (`self.LightRotation`)) false false)
  (`LightComponent.SetIntensity` (`self.PointLight`) (`self.IntensityPointLight`))
  (`LightComponent.SetLightColor` (`self.PointLight`) (`self.ColorPointLight`) true)
  (`LocalLightComponent.SetAttenuationRadius` (`self.PointLight`) (`self.AttenationRadius`)))