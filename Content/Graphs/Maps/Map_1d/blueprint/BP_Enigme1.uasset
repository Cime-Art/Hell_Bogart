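; BP_Enigme1 is an ordered three-brazier puzzle that opens PorteOuroboros when the player completes the sequence.
; Trigger boxes feed DoOnce-gated checks on prior braziers and the character's Fighting state, turning each point light green on success.
; A failed check at the second or third brazier flashes all lights red, then clears progress and re-arms the gates after a delay.
; Wwise events play feedback sounds and a completion music cue.
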(event `AudioEvent`
  (params (`green/red` :type Boolean))
  (bind _returnvalue (`GameplayStatics.GetPlayerCharacter` 0))
  ;[0.269 1 0.3029] AUDIO EVENT
  (if `green/red`
    (`AkGameplayStatics.PostEvent` "/Game/sound_design/Wwise/Environment/GroundSwitches/E_GroundSwitch_Low.E_GroundSwitch_Low" _returnvalue)
    (else
      (`AkGameplayStatics.PostEvent` "/Game/sound_design/Wwise/Environment/GroundSwitches/E_GroundSwitch_Medium.E_GroundSwitch_Medium" _returnvalue))))

(event `self.Box_1.OnComponentBeginOverlap`
  (params (OverlappedComponent :type "PrimitiveComponent Object Reference") (OtherActor :type "Actor Object Reference") (OtherComp :type "PrimitiveComponent Object Reference") (OtherBodyIndex :type Integer) (bFromSweep :type Boolean) (SweepResult :type "HitResult Structure (by ref)"))
  (bind _point_1 (`self.Point_1`))
  (bind _astop_down_character (cast `/Game/Prog/topDownBear/Blueprints/TopDownCharacter` OtherActor))
  (`/Engine/EditorBlueprintResources/StandardMacros.DoOnce` false :!label _label
    (:`Completed`
      (if (and (not (`/Game/Prog/topDownBear/Blueprints/TopDownCharacter.Fighting?` _astop_down_character)) (not (`self.Brasero1Lit?`)) (not (`self.EnigmaFailed?`)))
        ;[1 1 1] si vraie change la couleur et affiche, set le bool en vraie
        (`LightComponent.SetLightColor` _point_1 (struct :`R` 0.086993 :`G` 1.0 :`A` 1.0) true)
        (`SceneComponent.SetVisibility` _point_1 true false)
        (set `self.Brasero1Lit?` true)
        (`self.AudioEvent` true)
        (else
          (`self.ResetDoOnce`))))))

(event `ResetDoOnce`
  (bind _point_2 (`self.Point_2`))
  (bind _point_2_2 (`self.Point_2`))
  (bind _point_3 (`self.Point_3`))
  (bind _point_2_3 (`self.Point_2`))
  (`|ExecutionSequence`
    (:`then_0`
      (goto _label :!via `Reset`))
    (:`then_1`
      (goto _label_2 :!via `Reset`))
    (:`then_2`
      (goto _label_3 :!via `Reset`))))

(event `self.Box_2.OnComponentBeginOverlap`
  (params (OverlappedComponent :type "PrimitiveComponent Object Reference") (OtherActor :type "Actor Object Reference") (OtherComp :type "PrimitiveComponent Object Reference") (OtherBodyIndex :type Integer) (bFromSweep :type Boolean) (SweepResult :type "HitResult Structure (by ref)"))
  (bind _point_2 (`self.Point_2`))
  (bind _point_2_2 (`self.Point_2`))
  (bind _astop_down_character (cast `/Game/Prog/topDownBear/Blueprints/TopDownCharacter` OtherActor))
  (if (and (not (`self.Brasero2Lit?`)) (not (`self.EnigmaFailed?`)))
    (`/Engine/EditorBlueprintResources/StandardMacros.DoOnce` false :!label _label_2
      (:`Completed`
        (if (and (`self.Brasero1Lit?`) (not (`/Game/Prog/topDownBear/Blueprints/TopDownCharacter.Fighting?` _astop_down_character)))
          ;[1 1 1] si vraie change la couleur et affiche, set le bool en vraie
          (`LightComponent.SetLightColor` _point_2_2 (struct :`G` 1.0 :`B` 0.025844 :`A` 1.0) true)
          (`SceneComponent.SetVisibility` _point_2_2 true false)
          (set `self.Brasero2Lit?` true)
          (`self.AudioEvent` true)
          (else
            ;[1 1 1] Si brassero1 est  faux  allume tout en rouge pendant un temps puis eteint
            (set `self.EnigmaFailed?` true)
            (`LightComponent.SetLightColor` (`self.Point_1`) (struct :`R` 1.0 :`G` 0.005885 :`A` 1.0) true)
            (`LightComponent.SetLightColor` (`self.Point_3`) (struct :`R` 1.0 :`G` 0.005885 :`A` 1.0) true)
            (`LightComponent.SetLightColor` _point_2 (struct :`R` 1.0 :`G` 0.005885 :`A` 1.0) true)
            (`SceneComponent.SetVisibility` _point_2 true false)
            (`SceneComponent.SetVisibility` (`self.Point_3`) true false)
            (`SceneComponent.SetVisibility` (`self.Point_1`) true false)
            (`self.AudioEvent` false)
            (`KismetSystemLibrary.Delay` 3.0)
            (`SceneComponent.SetVisibility` _point_2 false false)
            (`SceneComponent.SetVisibility` (`self.Point_3`) false false)
            (`SceneComponent.SetVisibility` (`self.Point_1`) false false)
            (set `self.Brasero1Lit?` false)
            (set `self.EnigmaFailed?` false)
            (`self.ResetDoOnce`)))))))

(event `self.Box_3.OnComponentBeginOverlap`
  (params (OverlappedComponent :type "PrimitiveComponent Object Reference") (OtherActor :type "Actor Object Reference") (OtherComp :type "PrimitiveComponent Object Reference") (OtherBodyIndex :type Integer) (bFromSweep :type Boolean) (SweepResult :type "HitResult Structure (by ref)"))
  (bind _point_3 (`self.Point_3`))
  (bind _point_2 (`self.Point_2`))
  (bind _astop_down_character (cast `/Game/Prog/topDownBear/Blueprints/TopDownCharacter` OtherActor))
  (if (and (not (`self.Brasero3Lit?`)) (not (`self.EnigmaFailed?`)))
    (`/Engine/EditorBlueprintResources/StandardMacros.DoOnce` false :!label _label_3
      (:`Completed`
        (if (and (`self.Brasero1Lit?`) (`self.Brasero2Lit?`) (not (`/Game/Prog/topDownBear/Blueprints/TopDownCharacter.Fighting?` _astop_down_character)))
          ;[1 1 1] si vraie change la couleur et affiche, set le bool en vraie
          (`LightComponent.SetLightColor` _point_3 (struct :`G` 1.0 :`B` 0.025844 :`A` 1.0) true)
          (`SceneComponent.SetVisibility` _point_3 true false)
          (set `self.Brasero3Lit?` true)
          (`self.AudioEvent` true)
          (`AkGameplayStatics.PostEvent` "/Game/sound_design/Wwise/Music/Jungle/E_Mus_TriggerEnigme.E_Mus_TriggerEnigme" (`GameplayStatics.GetPlayerCharacter` 0))
          (`/Game/Graphs/Asset_Defs/Meshes/Structures/porte_oroboros/Porte_Oroboros_egnime2.OpenDoor` (`self.PorteOuroboros`))
          (else
            ;[1 1 1] Si brassero 1,2 est faux,  allume tout en rouge pendant un temps puis eteint
            (set `self.EnigmaFailed?` true)
            (`LightComponent.SetLightColor` (`self.Point_1`) (struct :`R` 1.0 :`G` 0.005885 :`A` 1.0) true)
            (`LightComponent.SetLightColor` (`self.Point_3`) (struct :`R` 1.0 :`G` 0.005885 :`A` 1.0) true)
            (`LightComponent.SetLightColor` _point_2 (struct :`R` 1.0 :`G` 0.005885 :`A` 1.0) true)
            (`SceneComponent.SetVisibility` _point_2 true false)
            (`SceneComponent.SetVisibility` (`self.Point_3`) true false)
            (`SceneComponent.SetVisibility` (`self.Point_1`) true false)
            (`self.AudioEvent` false)
            (`KismetSystemLibrary.Delay` 3.0)
            (`SceneComponent.SetVisibility` _point_2 false false)
            (`SceneComponent.SetVisibility` (`self.Point_3`) false false)
            (`SceneComponent.SetVisibility` (`self.Point_1`) false false)
            (set `self.Brasero1Lit?` false)
            (set `self.Brasero2Lit?` false)
            (set `self.EnigmaFailed?` false)
            (`self.ResetDoOnce`)))))))

(fn `UserConstructionScript`)