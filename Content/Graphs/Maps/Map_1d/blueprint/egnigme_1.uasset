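; Puzzle actor for Map_1d in which the player must light three braziers in order to open the Ouroboros door.
; Three box overlaps check for TopDownCharacter and the preceding Brassero flags, turning each point light green and setting its flag.
; The third success calls OpenDoor on PorteOuroboros.
; Any failed check at the second or third box flashes all lights red briefly, then hides them and clears preceding flags.
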(event `self.ReceiveTick`
  (params (DeltaSeconds :type "Float (single-precision)")))

(event `self.Box_1.OnComponentBeginOverlap`
  (params (OverlappedComponent :type "PrimitiveComponent Object Reference") (OtherActor :type "Actor Object Reference") (OtherComp :type "PrimitiveComponent Object Reference") (OtherBodyIndex :type Integer) (bFromSweep :type Boolean) (SweepResult :type "HitResult Structure (by ref)"))
  (bind _point_1 (`self.Point_1`))
  (if (`.bSuccess` (cast `/Game/Prog/topDownBear/Blueprints/TopDownCharacter` OtherActor :!pure true))
    ;[1 1 1] si vraie change la couleur et affiche, set le bool en vraie
    (`LightComponent.SetLightColor` _point_1 (struct :`R` 0.086993 :`G` 1.0 :`A` 1.0) true)
    (`SceneComponent.SetVisibility` _point_1 true false)
    (set `self.Brassero1` true)))

(event `self.Box_2.OnComponentBeginOverlap`
  (params (OverlappedComponent :type "PrimitiveComponent Object Reference") (OtherActor :type "Actor Object Reference") (OtherComp :type "PrimitiveComponent Object Reference") (OtherBodyIndex :type Integer) (bFromSweep :type Boolean) (SweepResult :type "HitResult Structure (by ref)"))
  (bind _point_2 (`self.Point_2`))
  (bind _point_2_2 (`self.Point_2`))
  (if (and (`.bSuccess` (cast `/Game/Prog/topDownBear/Blueprints/TopDownCharacter` OtherActor :!pure true)) (`self.Brassero1`))
    ;[1 1 1] si vraie change la couleur et affiche, set le bool en vraie
    (`LightComponent.SetLightColor` _point_2_2 (struct :`G` 1.0 :`B` 0.025844 :`A` 1.0) true)
    (`SceneComponent.SetVisibility` _point_2_2 true false)
    (set `self.Brassero2` true)
    (else
      ;[1 1 1] Si brassero1 est  faux  allume tout en rouge pendant un temps puis eteint
      (`LightComponent.SetLightColor` (`self.Point_1`) (struct :`R` 1.0 :`G` 0.005885 :`A` 1.0) true)
      (`LightComponent.SetLightColor` (`self.Point_3`) (struct :`R` 1.0 :`G` 0.005885 :`A` 1.0) true)
      (`LightComponent.SetLightColor` _point_2 (struct :`R` 1.0 :`G` 0.005885 :`A` 1.0) true)
      (`SceneComponent.SetVisibility` _point_2 true false)
      (`SceneComponent.SetVisibility` (`self.Point_3`) true false)
      (`SceneComponent.SetVisibility` (`self.Point_1`) true false)
      (`KismetSystemLibrary.Delay` 3.0)
      (`SceneComponent.SetVisibility` _point_2 false false)
      (`SceneComponent.SetVisibility` (`self.Point_3`) false false)
      (`SceneComponent.SetVisibility` (`self.Point_1`) false false)
      (set `self.Brassero1` false))))

(event `self.Box_3.OnComponentBeginOverlap`
  (params (OverlappedComponent :type "PrimitiveComponent Object Reference") (OtherActor :type "Actor Object Reference") (OtherComp :type "PrimitiveComponent Object Reference") (OtherBodyIndex :type Integer) (bFromSweep :type Boolean) (SweepResult :type "HitResult Structure (by ref)"))
  (bind _point_3 (`self.Point_3`))
  (bind _point_2 (`self.Point_2`))
  (if (and (`.bSuccess` (cast `/Game/Prog/topDownBear/Blueprints/TopDownCharacter` OtherActor :!pure true)) (`self.Brassero1`) (`self.Brassero2`))
    ;[1 1 1] si vraie change la couleur et affiche, set le bool en vraie
    (`LightComponent.SetLightColor` _point_3 (struct :`G` 1.0 :`B` 0.025844 :`A` 1.0) true)
    (`SceneComponent.SetVisibility` _point_3 true false)
    (set `self.Brassero3` true)
    (`/Game/Graphs/Asset_Defs/Meshes/Structures/porte_oroboros/Porte_Oroboros_egnime2.OpenDoor` (`self.PorteOuroboros`))
    (else
      ;[1 1 1] Si brassero 1,2 est faux,  allume tout en rouge pendant un temps puis eteint
      (`LightComponent.SetLightColor` (`self.Point_1`) (struct :`R` 1.0 :`G` 0.005885 :`A` 1.0) true)
      (`LightComponent.SetLightColor` (`self.Point_3`) (struct :`R` 1.0 :`G` 0.005885 :`A` 1.0) true)
      (`LightComponent.SetLightColor` _point_2 (struct :`R` 1.0 :`G` 0.005885 :`A` 1.0) true)
      (`SceneComponent.SetVisibility` _point_2 true false)
      (`SceneComponent.SetVisibility` (`self.Point_3`) true false)
      (`SceneComponent.SetVisibility` (`self.Point_1`) true false)
      (`KismetSystemLibrary.Delay` 3.0)
      (`SceneComponent.SetVisibility` _point_2 false false)
      (`SceneComponent.SetVisibility` (`self.Point_3`) false false)
      (`SceneComponent.SetVisibility` (`self.Point_1`) false false)
      (set `self.Brassero1` false)
      (set `self.Brassero2` false))))

(fn `UserConstructionScript`)