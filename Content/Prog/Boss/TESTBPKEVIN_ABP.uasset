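; Test actor Blueprint that plays the Kali boss death effect as soon as play begins.
; It plays the death animation once on the skeletal mesh, then after a short delay spawns an attached Niagara system and shortly deactivates the other Niagara components.
; In parallel, it creates dynamic instances of four mesh materials and a timeline drives their Dissolve parameter.
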(event `self.ReceiveBeginPlay`
  (bind _sm_kali (`self.SM_Kali`))
  (bind _sm_kali_2 (`self.SM_Kali`))
  (bind _sm_kali_3 (`self.SM_Kali`))
  (bind _sm_kali_4 (`self.SM_Kali`))
  (`SkeletalMeshComponent.PlayAnimation` (`self.SM_Kali`) "/Game/Prog/Boss/Animations/Mort/Anim_Kali_Mort.Anim_Kali_Mort" false)
  (`|ExecutionSequence`
    (:`then_0`
      (`KismetSystemLibrary.Delay` 0.95)
      (`NiagaraFunctionLibrary.SpawnSystemAttached` "/Game/Prog/Boss/TestDissolve/SkeletalMeshSystem.SkeletalMeshSystem" (`self.SM_Kali`) "None" (0.0 0.0 0.0) (struct) "KeepRelativeOffset")
      (`KismetSystemLibrary.Delay` 0.1)
      (`ActorComponent.SetActive` (`self.Niagara`) false false)
      (`ActorComponent.SetActive` (`self.Niagara2`) false false)
      (`ActorComponent.SetActive` (`self.Niagara3`) false false)
      (`ActorComponent.SetActive` (`self.Niagara4`) false false)
      (`ActorComponent.SetActive` (`self.Niagara1`) false false)
      (`ActorComponent.SetActive` (`self.Niagara5`) false false))
    (:`then_1`
      (bind _returnvalue (`PrimitiveComponent.CreateDynamicMaterialInstance` _sm_kali_3 0 (`PrimitiveComponent.GetMaterial` _sm_kali_3 0) "D1"))
      (`PrimitiveComponent.SetMaterial` _sm_kali_3 0 _returnvalue))
    (:`then_2`
      (bind _returnvalue_2 (`PrimitiveComponent.CreateDynamicMaterialInstance` _sm_kali_4 1 (`PrimitiveComponent.GetMaterial` _sm_kali_4 1) "D2"))
      (`PrimitiveComponent.SetMaterial` _sm_kali_4 1 _returnvalue_2))
    (:`then_3`
      (bind _returnvalue_3 (`PrimitiveComponent.CreateDynamicMaterialInstance` _sm_kali 3 (`PrimitiveComponent.GetMaterial` _sm_kali 3) "3"))
      (`PrimitiveComponent.SetMaterial` _sm_kali 3 _returnvalue_3))
    (:`then_4`
      (bind _returnvalue_4 (`PrimitiveComponent.CreateDynamicMaterialInstance` _sm_kali_2 2 (`PrimitiveComponent.GetMaterial` _sm_kali_2 2) "D4"))
      (`PrimitiveComponent.SetMaterial` _sm_kali_2 2 _returnvalue_4)
      (bind (_direction _newtrack_0) (`Timeline|Dissolve_Time`)
        (:`Update`
          (`MaterialInstanceDynamic.SetScalarParameterValue` _returnvalue_4 "Dissolve" _newtrack_0)
          (`MaterialInstanceDynamic.SetScalarParameterValue` _returnvalue_3 "Dissolve" _newtrack_0)
          (`MaterialInstanceDynamic.SetScalarParameterValue` _returnvalue_2 "Dissolve" _newtrack_0)
          (`MaterialInstanceDynamic.SetScalarParameterValue` _returnvalue "Dissolve" _newtrack_0))))))

(fn `UserConstructionScript`)