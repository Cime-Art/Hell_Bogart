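; Falling-rocks event actor that drops a destructible when the TopDownCharacter enters its trigger box.
; The overlap turns on physics, and the destructible's first hit fires a radial force impulse and posts a Wwise wall-destruction sound on the player pawn.
; That hit also sets Finished, updates the game instance and destroys the actor after a short delay.
; The AlreadyFinished event destroys the actor immediately.
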(event `self.Box.OnComponentBeginOverlap`
  (params (OverlappedComponent :type "PrimitiveComponent Object Reference") (OtherActor :type "Actor Object Reference") (OtherComp :type "PrimitiveComponent Object Reference") (OtherBodyIndex :type Integer) (bFromSweep :type Boolean) (SweepResult :type "HitResult Structure (by ref)"))
  (cast `/Game/Prog/topDownBear/Blueprints/TopDownCharacter` OtherActor)
  (`PrimitiveComponent.SetSimulatePhysics` (`self.Destructible`) true))

(event `self.Destructible.OnComponentHit`
  (params (HitComponent :type "PrimitiveComponent Object Reference") (OtherActor :type "Actor Object Reference") (OtherComp :type "PrimitiveComponent Object Reference") (NormalImpulse :type "Vector Structure") (Hit :type "HitResult Structure (by ref)"))
  (bind _returnvalue (`GameplayStatics.GetPlayerPawn` 0))
  (`/Engine/EditorBlueprintResources/StandardMacros.DoOnce` false
    (:`Completed`
      (`RadialForceComponent.FireImpulse` (`self.RadialForce`))
      (`AkGameplayStatics.SetSwitch` "Destroyed_Object_Type_SWITCH" "Walls" _returnvalue)
      (`AkGameplayStatics.PostEvent` "/Game/sound_design/Wwise/Environment/Destructibles/E_Destroy_Object.E_Destroy_Object" _returnvalue)
      (set `self.?Finished` true)
      (`self.UpdateGameInstance`)
      (`KismetSystemLibrary.Delay` 5.0)
      (`self.K2_DestroyActor`))))

(event `self.AlreadyFinished`
  (`self.K2_DestroyActor`))

(fn `UserConstructionScript`
  (`parent.UserConstructionScript`))