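; Destructible prop actor that shows a configurable Mesh and cleans up its debris after fracturing.
; The construction script and a SetMesh event assign the mesh to the destructible component.
; On fracture, the first five characters of the mesh's name set a Wwise switch for the destroy sound.
; It then changes collision profile and chunk threshold, waits TimeToDespawn, dissolves materials through a timeline and destroys itself.
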(event `self.Destructible.OnComponentFracture`
  (params (HitPoint :type "Vector Structure (by ref)") (HitDirection :type "Vector Structure (by ref)"))
  (bind _destructible (`self.Destructible`))
  (`AkGameplayStatics.SetSwitch` "Destroyed_Object_Type_SWITCH" (`KismetStringLibrary.Conv_StringToName` (`KismetStringLibrary.GetSubstring` (`KismetSystemLibrary.GetDisplayName` (`self.mesh`)) 0 5)) self)
  (`AkGameplayStatics.PostEvent` "/Game/sound_design/Wwise/Environment/Destructibles/E_Destroy_Object.E_Destroy_Object" self)
  (`PrimitiveComponent.SetCollisionProfileName` _destructible "EndDestroy")
  (set `DestructibleComponent.LargeChunkThreshold` 10000.0 _destructible)
  ;[0 1 0.009654] A modifier pour fade l'opacité des débris avant destruction
  (`KismetSystemLibrary.Delay` (`self.timeToDespawn`))
  (bind (_direction _time_to_disolve) (`Timeline|disolve`)
    (:`Update`
      (`MeshComponent.SetScalarParameterValueOnMaterials` (`self.Destructible`) "Amount" _time_to_disolve))
    (:`Finished`
      (`self.K2_DestroyActor`))))

(event `SetMesh`
  (`DestructibleComponent.SetDestructibleMesh` (`self.Destructible`) (`self.mesh`)))

(fn `UserConstructionScript`
  (`DestructibleComponent.SetDestructibleMesh` (`self.Destructible`) (`self.mesh`)))