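; Item loot spawner that rolls a percentage drop chance for each item and spawns winners as BP_Item actors, initialized with speed and chest reference.
; The splitItem macro sorts item names by substring into weapon mods, grenade, medkit or treasure, using boolean flags to allow one per category.
; Unrecognized names print an error.
; When the 1MIN flag is set, the roll repeats after a short delay until something passes.
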(event `ItemLoot`
  (params (X1 :type "Map of Name to Boolean") (item :type "Map of Name to Float (double-precision) (by ref)") (spawn :type "Vector Structure") (speed :type "Float (double-precision)") (`1MIN` :type Boolean) (chestRef :type "/Game/Prog/blueprint/Coffre/BP_Coffre Object Reference"))
  (bind _values (`BlueprintMapLibrary.Map_Values` X1))
  (bind _keys (`BlueprintMapLibrary.Map_Keys` item))
  (for _array_element _keys :!label _label
    (if (<= (`KismetMathLibrary.RandomFloatInRange` 0.0 100.0) (`BlueprintMapLibrary.Map_Find` item _array_element))
      (set `self.isActif?` true)
      (`self.splitItem` (`KismetStringLibrary.Conv_NameToString` _array_element) _values
        (:`modsArme`
          _)
        (:`grenade`
          _)
        (:`medikit`
          _)
        (:`tresor`
          _))
      (bind _returnvalue (`|SpawnActorFromClass` "/Game/Prog/blueprint/items/BP_Item.BP_Item_C" (`KismetMathLibrary.MakeTransform` spawn) "AdjustIfPossibleButAlwaysSpawn" "OverrideRootScale" null null))
      (set `/Game/Prog/blueprint/items/BP_Item.itemName` _array_element _returnvalue)
      (`/Game/Prog/blueprint/items/BP_Item.creation` _returnvalue speed chestRef)))
  (`KismetSystemLibrary.Delay` 0.1)
  (if (and `1MIN` (not (`self.isActif?`)))
    (`KismetSystemLibrary.PrintString` "retry : not spawn")
    (goto _label)))