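; Explosive shot actor that detonates when its Sphere overlaps a BP_Ennemy or after a two-second timer accumulated in Tick.
; Detonation switches RadiusExplo to overlap collision, resizes it to SphereRadius, spawns a grenade explosion emitter and destroys the actor after a short delay.
; The resulting RadiusExplo overlaps call GetDamage on each enemy, passing damage, the shot itself and explosion force.
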(event `self.ReceiveTick`
  (params (DeltaSeconds :type "Float (single-precision)"))
  (bind _output_get (set `self.timerSelfExplo` (+ DeltaSeconds (`self.timerSelfExplo`))))
  (if (>= _output_get 2.0)
    (`PrimitiveComponent.SetCollisionProfileName` (`self.radiusExplo`) "OverlapAllDynamic")
    (`SphereComponent.SetSphereRadius` (`self.radiusExplo`) (`self.sphereRadius`) true)
    (`GameplayStatics.SpawnEmitterAtLocation` "/Game/Prog/PrototypeWeap/FX/P_GrenadeLauncher_Explosion_01.P_GrenadeLauncher_Explosion_01" (`self.K2_GetActorLocation`))
    (`KismetSystemLibrary.Delay` 0.1)
    (`self.K2_DestroyActor`)))

(event `self.radiusExplo.OnComponentBeginOverlap`
  (params (OverlappedComponent :type "PrimitiveComponent Object Reference") (OtherActor :type "Actor Object Reference") (OtherComp :type "PrimitiveComponent Object Reference") (OtherBodyIndex :type Integer) (bFromSweep :type Boolean) (SweepResult :type "HitResult Structure (by ref)"))
  (bind _asbp_ennemy (cast `/Game/Prog/blueprint/IA/BP_Ennemy` OtherActor))
  (`/Game/Prog/blueprint/IA/BP_Ennemy.GetDamage` _asbp_ennemy (`self.Damage`) self null (`self.forceExplo`) (0.0 0.0 0.0)))

(event `self.Sphere.OnComponentBeginOverlap`
  (params (OverlappedComponent :type "PrimitiveComponent Object Reference") (OtherActor :type "Actor Object Reference") (OtherComp :type "PrimitiveComponent Object Reference") (OtherBodyIndex :type Integer) (bFromSweep :type Boolean) (SweepResult :type "HitResult Structure (by ref)"))
  (cast `/Game/Prog/blueprint/IA/BP_Ennemy` OtherActor)
  (`PrimitiveComponent.SetCollisionProfileName` (`self.radiusExplo`) "OverlapAllDynamic")
  (`SphereComponent.SetSphereRadius` (`self.radiusExplo`) (`self.sphereRadius`) true)
  (`GameplayStatics.SpawnEmitterAtLocation` "/Game/Prog/PrototypeWeap/FX/P_GrenadeLauncher_Explosion_01.P_GrenadeLauncher_Explosion_01" (`self.K2_GetActorLocation`))
  (`KismetSystemLibrary.Delay` 0.1)
  (`self.K2_DestroyActor`))

(fn `UserConstructionScript`)