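; BP_EventGatling is a one-shot trigger that stages the player's first Gatling event.
; When a TopDownCharacter first enters its Box, it sets the character's FirstTimeGatling flag and turns them toward the LookAt component.
; It then freezes gameplay through zero global time dilation and posts a Wwise time-dilation event, with global low-pass and pitch RTPCs interpolated for the slowdown effect.
; Nothing here restores time or audio.
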(event `self.Box.OnComponentBeginOverlap`
  (params (OverlappedComponent :type "PrimitiveComponent Object Reference") (OtherActor :type "Actor Object Reference") (OtherComp :type "PrimitiveComponent Object Reference") (OtherBodyIndex :type Integer) (bFromSweep :type Boolean) (SweepResult :type "HitResult Structure (by ref)"))
  (bind _astop_down_character (cast `/Game/Prog/topDownBear/Blueprints/TopDownCharacter` OtherActor))
  (`/Engine/EditorBlueprintResources/StandardMacros.DoOnce` false
    (:`Completed`
      (set `/Game/Prog/topDownBear/Blueprints/TopDownCharacter.firstTimeGatling` true _astop_down_character)
      (`self.K2_SetActorRotation` _astop_down_character (`KismetMathLibrary.FindLookAtRotation` (`self.K2_GetActorLocation` _astop_down_character) (`SceneComponent.K2_GetComponentLocation` (`self.LookAt`))) false)
      (`GameplayStatics.SetGlobalTimeDilation` 0.0)
      (`AkGameplayStatics.PostEvent` "/Game/sound_design/Wwise/Global/E_Global_TimeDilatation_On.E_Global_TimeDilatation_On" (`GameplayStatics.GetPlayerPawn` 0))
      (`AkGameplayStatics.SetRTPCValue` "LowPassGlobal_GP" 70.0 200)
      (`AkGameplayStatics.SetRTPCValue` "PitchGlobal_GP" -3000.0 1000))))

(fn `UserConstructionScript`
  (`parent.UserConstructionScript`))