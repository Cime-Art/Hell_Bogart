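; Double stone door for a buffer zone ("ZoneTampon") that swings open once when a TopDownCharacter enters its trigger box.
; Timelines rotate the two leaves in opposite yaw directions from angles cached at BeginPlay, with Wwise events for opening and stop.
; The Reverse flag selects a second timeline with a narrower swing, bracketed by DisableInput/EnableInput calls on the door itself.
; The construction script sizes the trigger from an extent variable.
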(event `self.ReceiveBeginPlay`
  (bind (_returnvalue_roll _returnvalue_pitch _returnvalue_yaw) (`KismetMathLibrary.BreakRotator` (`SceneComponent.K2_GetComponentRotation` (`self.porte_droite`))))
  (bind (_returnvalue_roll_2 _returnvalue_pitch_2 _returnvalue_yaw_2) (`KismetMathLibrary.BreakRotator` (`SceneComponent.K2_GetComponentRotation` (`self.porte_gauche`))))
  (set `self.originalYaw_PorteDroite` _returnvalue_yaw)
  (set `self.originalYaw_PorteGauche` _returnvalue_yaw_2))

(event `self.TB_Start.OnComponentBeginOverlap`
  (params (OverlappedComponent :type "PrimitiveComponent Object Reference") (OtherActor :type "Actor Object Reference") (OtherComp :type "PrimitiveComponent Object Reference") (OtherBodyIndex :type Integer) (bFromSweep :type Boolean) (SweepResult :type "HitResult Structure (by ref)"))
  (bind _originalyaw_portegauche (`self.originalYaw_PorteGauche`))
  (bind _originalyaw_portedroite (`self.originalYaw_PorteDroite`))
  (bind _originalyaw_portegauche_2 (`self.originalYaw_PorteGauche`))
  (bind _originalyaw_portedroite_2 (`self.originalYaw_PorteDroite`))
  (`KismetSystemLibrary.Delay` 0.0)
  (cast `/Game/Prog/topDownBear/Blueprints/TopDownCharacter` OtherActor)
  (`/Engine/EditorBlueprintResources/StandardMacros.DoOnce` false
    (:`Completed`
      (`AkGameplayStatics.PostEvent` "/Game/sound_design/Wwise/Global/E_Enable_Attenuation.E_Enable_Attenuation" self)
      ;[1 1 1] Event do not start
      (`AkGameplayStatics.PostEvent` "/Game/sound_design/Wwise/Environment/BigStoneDoor/E_BigStoneDoor_Opening.E_BigStoneDoor_Opening" self)
      (if (not (`self.reverse`))
        (bind (_direction _alpha) (`Timeline|OpenDoors` :!via `PlayFromStart`)
          (:`Update`
            (`SceneComponent.K2_SetWorldRotation` (`self.porte_droite`) (`KismetMathLibrary.MakeRotator` 0.0 0.0 (`KismetMathLibrary.MapRangeClamped` _alpha 0.0 1.0 _originalyaw_portedroite_2 (+ _originalyaw_portedroite_2 80.0))) false false)
            (`SceneComponent.K2_SetWorldRotation` (`self.porte_gauche`) (`KismetMathLibrary.MakeRotator` 0.0 0.0 (`KismetMathLibrary.MapRangeClamped` _alpha 0.0 1.0 _originalyaw_portegauche (- _originalyaw_portegauche 80.0))) false false))
          (:`Finished`
            (`AkGameplayStatics.PostEvent` "/Game/sound_design/Wwise/Environment/BigStoneDoor/E_BigStoneDoor_Stop.E_BigStoneDoor_Stop" self)))
        (else
          (`self.DisableInput` self (`GameplayStatics.GetPlayerController` 0))
          (bind (_direction_2 _alpha_2) (`Timeline|Timeline_0` :!via `PlayFromStart`)
            (:`Update`
              (`SceneComponent.K2_SetWorldRotation` (`self.porte_droite`) (`KismetMathLibrary.MakeRotator` 0.0 0.0 (`KismetMathLibrary.MapRangeClamped` _alpha_2 0.0 1.0 _originalyaw_portedroite (+ _originalyaw_portedroite 60.0))) false false)
              (`SceneComponent.K2_SetWorldRotation` (`self.porte_gauche`) (`KismetMathLibrary.MakeRotator` 0.0 0.0 (`KismetMathLibrary.MapRangeClamped` _alpha_2 0.0 1.0 _originalyaw_portegauche_2 (- _originalyaw_portegauche_2 60.0))) false false))
            (:`Finished`
              (`AkGameplayStatics.PostEvent` "/Game/sound_design/Wwise/Environment/BigStoneDoor/E_BigStoneDoor_Stop.E_BigStoneDoor_Stop" self)
              (`self.EnableInput` self (`GameplayStatics.GetPlayerController` 0)))))))))

(fn `UserConstructionScript`
  (`BoxComponent.SetBoxExtent` (`self.TB_Start`) (`self.boxExtent_TriggerBox`) true))