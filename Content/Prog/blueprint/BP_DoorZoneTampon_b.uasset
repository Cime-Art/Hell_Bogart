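; Buffer-zone double stone door that swings open when the TopDownCharacter enters its trigger box.
; The overlap plays a timeline from the start, adding opposite yaw to the right and left leaves on each update, so rotation accumulates rather than interpolating to a target.
; Wwise events play the opening sound and a stop sound when the timeline finishes.
; The construction script sizes the trigger box from a variable.
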(event `self.TB_Start.OnComponentBeginOverlap`
  (params (OverlappedComponent :type "PrimitiveComponent Object Reference") (OtherActor :type "Actor Object Reference") (OtherComp :type "PrimitiveComponent Object Reference") (OtherBodyIndex :type Integer) (bFromSweep :type Boolean) (SweepResult :type "HitResult Structure (by ref)"))
  (cast `/Game/Prog/topDownBear/Blueprints/TopDownCharacter` OtherActor)
  ;[1 1 1] Event do not start
  (`AkGameplayStatics.PostEvent` "/Game/sound_design/Wwise/Environment/BigStoneDoor/E_BigStoneDoor_Opening.E_BigStoneDoor_Opening" self)
  (bind (_direction _alpha) (`Timeline|OpenDoors` :!via `PlayFromStart`)
    (:`Update`
      (bind _returnvalue (* _alpha 1.0))
      (`SceneComponent.K2_AddWorldRotation` (`self.porte_droite`) (`KismetMathLibrary.MakeRotator` 0.0 0.0 _returnvalue) false false)
      (`SceneComponent.K2_AddWorldRotation` (`self.porte_gauche`) (`KismetMathLibrary.MakeRotator` 0.0 0.0 (* _returnvalue -1.0)) false false))
    (:`Finished`
      (`AkGameplayStatics.PostEvent` "/Game/sound_design/Wwise/Environment/BigStoneDoor/E_BigStoneDoor_Stop.E_BigStoneDoor_Stop" self))))

(fn `UserConstructionScript`
  (`BoxComponent.SetBoxExtent` (`self.TB_Start`) (`self.boxExtent_TriggerBox`) true))