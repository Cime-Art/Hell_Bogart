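; Camera zone that zooms the top-down player's view on entering a radius-driven sphere and reverses it on exit, with sound cues.
; A timeline blends spring arm length, arm rotation and camera rotation from default to zone settings.
; The first entry locks movement and input until the blend finishes.
; Zone ID selects Wwise events: a one-time bear line, or bridge music phases, the last triggered by a box overlap.
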(event `self.Sphere.OnComponentBeginOverlap`
  (params (OverlappedComponent :type "PrimitiveComponent Object Reference") (OtherActor :type "Actor Object Reference") (OtherComp :type "PrimitiveComponent Object Reference") (OtherBodyIndex :type Integer) (bFromSweep :type Boolean) (SweepResult :type "HitResult Structure (by ref)"))
  (bind (_settings_armlength _settings_armrotation _settings_camerarotation) (break `/Game/Prog/blueprint/Camera/SpringArm_Camera_Settings` (`self.Settings`)))
  (bind (_defaultplayersettings_armlength _defaultplayersettings_armrotation _defaultplayersettings_camerarotation) (break `/Game/Prog/blueprint/Camera/SpringArm_Camera_Settings` (`self.DefaultPlayerSettings`)))
  (bind _refplayer (`self.refPlayer`))
  (bind _refplayer_2 (`self.refPlayer`))
  (bind _refplayer_3 (`self.refPlayer`))
  (bind _refplayer_4 (`self.refPlayer`))
  (bind _roll (.roll _defaultplayersettings_armrotation))
  (bind _pitch (.pitch _defaultplayersettings_armrotation))
  (bind _yaw (.yaw _defaultplayersettings_armrotation))
  (bind _roll_2 (.roll _defaultplayersettings_camerarotation))
  (bind _pitch_2 (.pitch _defaultplayersettings_camerarotation))
  (bind _yaw_2 (.yaw _defaultplayersettings_camerarotation))
  (bind _astop_down_character (cast `/Game/Prog/topDownBear/Blueprints/TopDownCharacter` OtherActor))
  (set `self.refPlayer` _astop_down_character)
  (`|ExecutionSequence`
    (:`then_0`
      (`/Engine/EditorBlueprintResources/StandardMacros.DoOnce` false :!label _label
        (:`Completed`
          (set `self.zoom/dezoom` true)
          (if (== (`self.ID`) 2)
            (if (not (`/Game/Prog/topDownBear/Blueprints/TopDownCharacter.MusicBridge` _refplayer_3))
              (`AkGameplayStatics.PostEvent` "/Game/sound_design/Wwise/Music/Bridge/E_Mus_Bridge_Begin.E_Mus_Bridge_Begin" _refplayer_3)
              (set `/Game/Prog/topDownBear/Blueprints/TopDownCharacter.MusicBridge` true _refplayer_3)))
          (`|ExecutionSequence`
            (:`then_0`
              (`/Engine/EditorBlueprintResources/StandardMacros.DoOnce` false
                (:`Completed`
                  (`ActorComponent.Deactivate` (`Character.CharacterMovement` _refplayer_2))
                  (`self.DisableInput` _refplayer_2 (`GameplayStatics.GetPlayerController` 0))
                  (set `/Game/Prog/topDownBear/Blueprints/TopDownCharacter.addScreen` true _refplayer_2)
                  (bind (_direction _alpha) (`Timeline|Timeline_0` :!via `PlayFromStart` :!label _label_2)
                    (:`Update`
                      (set `SpringArmComponent.TargetArmLength` (+ (/ (* (- _settings_armlength _defaultplayersettings_armlength) _alpha) 100.0) _defaultplayersettings_armlength) (`/Game/Prog/topDownBear/Blueprints/TopDownCharacter.SpringArm` _refplayer))
                      (`SceneComponent.K2_SetRelativeRotation` (`/Game/Prog/topDownBear/Blueprints/TopDownCharacter.SpringArm` _refplayer) (`KismetMathLibrary.MakeRotator` (+ (/ (* (- (.roll _settings_armrotation) _roll) _alpha) 100.0) _roll) (+ (/ (* (- (.pitch _settings_armrotation) _pitch) _alpha) 100.0) _pitch) (+ (/ (* (- (.yaw _settings_armrotation) _yaw) _alpha) 100.0) _yaw)) false false)
                      (`SceneComponent.K2_SetRelativeRotation` (`/Game/Prog/topDownBear/Blueprints/TopDownCharacter.Camera` _refplayer) (`KismetMathLibrary.MakeRotator` (+ (/ (* (- (.roll _settings_camerarotation) _roll_2) _alpha) 100.0) _roll_2) (+ (/ (* (- (.pitch _settings_camerarotation) _pitch_2) _alpha) 100.0) _pitch_2) (+ (/ (* (- (.yaw _settings_camerarotation) _yaw_2) _alpha) 100.0) _yaw_2)) false false))
                    (:`Finished`
                      (if (`self.zoom/dezoom`)
                        (if (== (`self.ID`) 0)
                          (`/Engine/EditorBlueprintResources/StandardMacros.DoOnce` false
                            (:`Completed`
                              (`AkGameplayStatics.PostEvent` "/Game/sound_design/Wwise/Voice/Bear/EXPLO/E_Speech_Bear_EXPLO_ItsBeautiful_PRIORITY.E_Speech_Bear_EXPLO_ItsBeautiful_PRIORITY" _refplayer_4))))
                        (`ActorComponent.Activate` (`Character.CharacterMovement` _refplayer_4) false)
                        (`self.EnableInput` _refplayer_4 (`GameplayStatics.GetPlayerController` 0))
                        (set `/Game/Prog/topDownBear/Blueprints/TopDownCharacter.addScreen` false _refplayer_4)
                        (if (and (not (`/Game/Prog/topDownBear/Blueprints/TopDownCharacter.BridgePhase1` _refplayer_4)) (== (`self.ID`) 2) (`/Game/Prog/topDownBear/Blueprints/TopDownCharacter.MusicBridge` _refplayer_4))
                          (`AkGameplayStatics.PostEvent` "/Game/sound_design/Wwise/Music/Bridge/E_Mus_Bridge_GoToPhase1.E_Mus_Bridge_GoToPhase1" _refplayer_4)
                          (set `/Game/Prog/topDownBear/Blueprints/TopDownCharacter.BridgePhase1` true _refplayer_4))))))))
            (:`then_1`
              (goto _label_2 :!via `PlayFromStart`))))))
    (:`then_1`
      (goto _label_3 :!via `Reset`))))

(event `self.Sphere.OnComponentEndOverlap`
  (params (OverlappedComponent :type "PrimitiveComponent Object Reference") (OtherActor :type "Actor Object Reference") (OtherComp :type "PrimitiveComponent Object Reference") (OtherBodyIndex :type Integer))
  (cast `/Game/Prog/topDownBear/Blueprints/TopDownCharacter` OtherActor)
  (`|ExecutionSequence`
    (:`then_0`
      (`/Engine/EditorBlueprintResources/StandardMacros.DoOnce` false :!label _label_3
        (:`Completed`
          (set `self.zoom/dezoom` true)
          (goto _label_2 :!via `Reverse`))))
    (:`then_1`
      (goto _label :!via `Reset`))))

(event `self.Box.OnComponentBeginOverlap`
  (params (OverlappedComponent :type "PrimitiveComponent Object Reference") (OtherActor :type "Actor Object Reference") (OtherComp :type "PrimitiveComponent Object Reference") (OtherBodyIndex :type Integer) (bFromSweep :type Boolean) (SweepResult :type "HitResult Structure (by ref)"))
  (bind _astop_down_character (cast `/Game/Prog/topDownBear/Blueprints/TopDownCharacter` OtherActor))
  (if (== (`self.ID`) 2)
    (`/Engine/EditorBlueprintResources/StandardMacros.DoOnce` false
      (:`Completed`
        (`AkGameplayStatics.PostEvent` "/Game/sound_design/Wwise/Music/Bridge/E_Mus_Bridge_GoToPhase2.E_Mus_Bridge_GoToPhase2" _astop_down_character)))))

(fn `UserConstructionScript`
  (`SphereComponent.SetSphereRadius` (`self.Sphere`) (`self.Radius`) true))