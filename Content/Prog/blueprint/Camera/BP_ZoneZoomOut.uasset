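; Camera zone that blends the TopDownCharacter's spring arm and camera to zone Settings inside a radius-sized sphere, and back to defaults on exit.
; Two timelines drive the interpolation, with paired DoOnce gates re-arming each other on overlap begin and end.
; It also drives Wwise bridge music: the first zoom pauses movement until finished, then starts the music; a later zoom triggers phase 1, and a separate box triggers phase 2 once.
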(event `self.Sphere.OnComponentBeginOverlap`
  (params (OverlappedComponent :type "PrimitiveComponent Object Reference") (OtherActor :type "Actor Object Reference") (OtherComp :type "PrimitiveComponent Object Reference") (OtherBodyIndex :type Integer) (bFromSweep :type Boolean) (SweepResult :type "HitResult Structure (by ref)"))
  (bind (_settings_armlength _settings_armrotation _settings_camerarotation) (break `/Game/Prog/blueprint/Camera/SpringArm_Camera_Settings` (`self.Settings`)))
  (bind (_defaultplayersettings_armlength _defaultplayersettings_armrotation _defaultplayersettings_camerarotation) (break `/Game/Prog/blueprint/Camera/SpringArm_Camera_Settings` (`self.DefaultPlayerSettings`)))
  (bind (_settings_armlength_2 _settings_armrotation_2 _settings_camerarotation_2) (break `/Game/Prog/blueprint/Camera/SpringArm_Camera_Settings` (`self.Settings`)))
  (bind (_defaultplayersettings_armlength_2 _defaultplayersettings_armrotation_2 _defaultplayersettings_camerarotation_2) (break `/Game/Prog/blueprint/Camera/SpringArm_Camera_Settings` (`self.DefaultPlayerSettings`)))
  (bind _roll (.roll _settings_armrotation_2))
  (bind _pitch (.pitch _settings_armrotation_2))
  (bind _yaw (.yaw _settings_armrotation_2))
  (bind _roll_2 (.roll _settings_camerarotation_2))
  (bind _pitch_2 (.pitch _settings_camerarotation_2))
  (bind _yaw_2 (.yaw _settings_camerarotation_2))
  (bind _roll_3 (.roll _defaultplayersettings_armrotation))
  (bind _pitch_3 (.pitch _defaultplayersettings_armrotation))
  (bind _yaw_3 (.yaw _defaultplayersettings_armrotation))
  (bind _roll_4 (.roll _defaultplayersettings_camerarotation))
  (bind _pitch_4 (.pitch _defaultplayersettings_camerarotation))
  (bind _yaw_4 (.yaw _defaultplayersettings_camerarotation))
  (bind _astop_down_character (cast `/Game/Prog/topDownBear/Blueprints/TopDownCharacter` OtherActor))
  (`|ExecutionSequence`
    (:`then_0`
      (`/Engine/EditorBlueprintResources/StandardMacros.DoOnce` false :!label _label
        (:`Completed`
          (if (`/Game/Prog/topDownBear/Blueprints/TopDownCharacter.MusicBridge` _astop_down_character)
            (bind (_direction _alpha) (`Timeline|Timeline_0` :!via `PlayFromStart` :!label _label_2)
              (:`Update`
                (bind _springarm (`/Game/Prog/topDownBear/Blueprints/TopDownCharacter.SpringArm` _astop_down_character))
                (set `SpringArmComponent.TargetArmLength` (+ (/ (* (- _settings_armlength _defaultplayersettings_armlength) _alpha) 100.0) _defaultplayersettings_armlength) _springarm)
                (`SceneComponent.K2_SetRelativeRotation` _springarm (`KismetMathLibrary.MakeRotator` (+ (/ (* (- (.roll _settings_armrotation) _roll_3) _alpha) 100.0) _roll_3) (+ (/ (* (- (.pitch _settings_armrotation) _pitch_3) _alpha) 100.0) _pitch_3) (+ (/ (* (- (.yaw _settings_armrotation) _yaw_3) _alpha) 100.0) _yaw_3)) false false)
                (`SceneComponent.K2_SetRelativeRotation` (`/Game/Prog/topDownBear/Blueprints/TopDownCharacter.Camera` _astop_down_character) (`KismetMathLibrary.MakeRotator` (+ (/ (* (- (.roll _settings_camerarotation) _roll_4) _alpha) 100.0) _roll_4) (+ (/ (* (- (.pitch _settings_camerarotation) _pitch_4) _alpha) 100.0) _pitch_4) (+ (/ (* (- (.yaw _settings_camerarotation) _yaw_4) _alpha) 100.0) _yaw_4)) false false))
              (:`Finished`
                (if (`/Game/Prog/topDownBear/Blueprints/TopDownCharacter.MusicBridge` _astop_down_character)
                  (if (not (`/Game/Prog/topDownBear/Blueprints/TopDownCharacter.BridgePhase1` _astop_down_character))
                    (`AkGameplayStatics.PostEvent` "/Game/sound_design/Wwise/Music/Bridge/E_Mus_Bridge_GoToPhase1.E_Mus_Bridge_GoToPhase1" _astop_down_character)
                    (set `/Game/Prog/topDownBear/Blueprints/TopDownCharacter.BridgePhase1` true _astop_down_character))
                  (else
                    (`ActorComponent.Activate` (`Character.CharacterMovement` _astop_down_character) false)
                    (`AkGameplayStatics.PostEvent` "/Game/sound_design/Wwise/Music/Bridge/E_Mus_Bridge_Begin.E_Mus_Bridge_Begin" _astop_down_character)
                    (set `/Game/Prog/topDownBear/Blueprints/TopDownCharacter.MusicBridge` true _astop_down_character)))))
            (else
              (`ActorComponent.Deactivate` (`Character.CharacterMovement` _astop_down_character))
              (goto _label_2 :!via `PlayFromStart`))))))
    (:`then_1`
      (goto _label_3 :!via `Reset`))))

(event `self.Sphere.OnComponentEndOverlap`
  (params (OverlappedComponent :type "PrimitiveComponent Object Reference") (OtherActor :type "Actor Object Reference") (OtherComp :type "PrimitiveComponent Object Reference") (OtherBodyIndex :type Integer))
  (bind (_settings_armlength _settings_armrotation _settings_camerarotation) (break `/Game/Prog/blueprint/Camera/SpringArm_Camera_Settings` (`self.Settings`)))
  (bind (_defaultplayersettings_armlength _defaultplayersettings_armrotation _defaultplayersettings_camerarotation) (break `/Game/Prog/blueprint/Camera/SpringArm_Camera_Settings` (`self.DefaultPlayerSettings`)))
  (bind _roll (.roll _settings_armrotation))
  (bind _pitch (.pitch _settings_armrotation))
  (bind _yaw (.yaw _settings_armrotation))
  (bind _roll_2 (.roll _settings_camerarotation))
  (bind _pitch_2 (.pitch _settings_camerarotation))
  (bind _yaw_2 (.yaw _settings_camerarotation))
  (bind _astop_down_character (cast `/Game/Prog/topDownBear/Blueprints/TopDownCharacter` OtherActor))
  (`|ExecutionSequence`
    (:`then_0`
      (`/Engine/EditorBlueprintResources/StandardMacros.DoOnce` false :!label _label_3
        (:`Completed`
          (bind (_direction _alpha) (`Timeline|Timeline_1` :!via `PlayFromStart`)
            (:`Update`
              (bind _springarm (`/Game/Prog/topDownBear/Blueprints/TopDownCharacter.SpringArm` _astop_down_character))
              (set `SpringArmComponent.TargetArmLength` (+ (/ (* (- _defaultplayersettings_armlength _settings_armlength) _alpha) 100.0) _settings_armlength) _springarm)
              (`SceneComponent.K2_SetRelativeRotation` _springarm (`KismetMathLibrary.MakeRotator` (+ (/ (* (- (.roll _defaultplayersettings_armrotation) _roll) _alpha) 100.0) _roll) (+ (/ (* (- (.pitch _defaultplayersettings_armrotation) _pitch) _alpha) 100.0) _pitch) (+ (/ (* (- (.yaw _defaultplayersettings_armrotation) _yaw) _alpha) 100.0) _yaw)) false false)
              (`SceneComponent.K2_SetRelativeRotation` (`/Game/Prog/topDownBear/Blueprints/TopDownCharacter.Camera` _astop_down_character) (`KismetMathLibrary.MakeRotator` (+ (/ (* (- (.roll _defaultplayersettings_camerarotation) _roll_2) _alpha) 100.0) _roll_2) (+ (/ (* (- (.pitch _defaultplayersettings_camerarotation) _pitch_2) _alpha) 100.0) _pitch_2) (+ (/ (* (- (.yaw _defaultplayersettings_camerarotation) _yaw_2) _alpha) 100.0) _yaw_2)) false false))))))
    (:`then_1`
      (goto _label :!via `Reset`))))

(event `self.Box.OnComponentBeginOverlap`
  (params (OverlappedComponent :type "PrimitiveComponent Object Reference") (OtherActor :type "Actor Object Reference") (OtherComp :type "PrimitiveComponent Object Reference") (OtherBodyIndex :type Integer) (bFromSweep :type Boolean) (SweepResult :type "HitResult Structure (by ref)"))
  (bind _astop_down_character (cast `/Game/Prog/topDownBear/Blueprints/TopDownCharacter` OtherActor))
  (`/Engine/EditorBlueprintResources/StandardMacros.DoOnce` false
    (:`Completed`
      (`AkGameplayStatics.PostEvent` "/Game/sound_design/Wwise/Music/Bridge/E_Mus_Bridge_GoToPhase2.E_Mus_Bridge_GoToPhase2" _astop_down_character))))

(fn `UserConstructionScript`
  (`SphereComponent.SetSphereRadius` (`self.Sphere`) (`self.Radius`) true))