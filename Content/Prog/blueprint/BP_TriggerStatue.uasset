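; BP_TriggerStatue is a trigger volume that hides a statue and its pedestal while the TopDownCharacter is inside its box.
; Box begin and end overlap events switch off, then restore, visibility on the referenced Socle mesh and Statue root, without propagating to child components.
; The optional Couronne (crown) root follows the same toggle when its reference is valid.
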(event `self.Box.OnComponentBeginOverlap`
  (params (OverlappedComponent :type "PrimitiveComponent Object Reference") (OtherActor :type "Actor Object Reference") (OtherComp :type "PrimitiveComponent Object Reference") (OtherBodyIndex :type Integer) (bFromSweep :type Boolean) (SweepResult :type "HitResult Structure (by ref)"))
  (bind _staticmeshcomponent (`StaticMeshActor.StaticMeshComponent` (`self.socle`)))
  (cast `/Game/Prog/topDownBear/Blueprints/TopDownCharacter` OtherActor)
  (`/Engine/EditorBlueprintResources/StandardMacros.IsValid` (`self.couronne`)
    (:`Is Valid`
      (`SceneComponent.SetVisibility` _staticmeshcomponent false false)
      (`SceneComponent.SetVisibility` (`Actor.RootComponent` (`self.statue`)) false false)
      (`SceneComponent.SetVisibility` (`Actor.RootComponent` (`self.couronne`)) false false))
    (:`Is Not Valid`
      (`SceneComponent.SetVisibility` _staticmeshcomponent false false)
      (`SceneComponent.SetVisibility` (`Actor.RootComponent` (`self.statue`)) false false))))

(event `self.Box.OnComponentEndOverlap`
  (params (OverlappedComponent :type "PrimitiveComponent Object Reference") (OtherActor :type "Actor Object Reference") (OtherComp :type "PrimitiveComponent Object Reference") (OtherBodyIndex :type Integer))
  (bind _couronne (`self.couronne`))
  (cast `/Game/Prog/topDownBear/Blueprints/TopDownCharacter` OtherActor)
  (`/Engine/EditorBlueprintResources/StandardMacros.IsValid` _couronne
    (:`Is Valid`
      (`SceneComponent.SetVisibility` (`Actor.RootComponent` _couronne) true false)
      (`SceneComponent.SetVisibility` (`StaticMeshActor.StaticMeshComponent` (`self.socle`)) true false)
      (`SceneComponent.SetVisibility` (`Actor.RootComponent` (`self.statue`)) true false))
    (:`Is Not Valid`
      (`SceneComponent.SetVisibility` (`StaticMeshActor.StaticMeshComponent` (`self.socle`)) true false)
      (`SceneComponent.SetVisibility` (`Actor.RootComponent` (`self.statue`)) true false))))

(fn `UserConstructionScript`)