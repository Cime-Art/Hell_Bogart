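; TriggerBox_Rock is a trap trigger that drops or releases a rock when the player walks into it.
; When a TopDownCharacter overlaps DetectionZone, it disables that character's movement and enables physics simulation on the Sphere of the referenced Rock.
; It prints "Dead" as the only death feedback, with no damage or reset logic.
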(event `self.detectionZone.OnComponentBeginOverlap`
  (params (OverlappedComponent :type "PrimitiveComponent Object Reference") (OtherActor :type "Actor Object Reference") (OtherComp :type "PrimitiveComponent Object Reference") (OtherBodyIndex :type Integer) (bFromSweep :type Boolean) (SweepResult :type "HitResult Structure (by ref)"))
  (bind _astop_down_character (cast `/Game/Prog/topDownBear/Blueprints/TopDownCharacter` OtherActor))
  (`CharacterMovementComponent.DisableMovement` (`Character.CharacterMovement` _astop_down_character))
  (`PrimitiveComponent.SetSimulatePhysics` (`/Game/Prog/blueprint/Traps/Bp_Rolling_Rock.Sphere` (`self.rock`)) true)
  (`KismetSystemLibrary.PrintString` "Dead"))

(fn `UserConstructionScript`
  (`parent.UserConstructionScript`))