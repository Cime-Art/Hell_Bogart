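; Rolling rock trap that moves along the spline of a referenced track actor.
; On BeginPlay, a timeline scaled by a duration variable and begun at a start offset lerps distance along the spline to set the actor's location.
; Spline rotation is left unconnected, so the rock does not follow the track's orientation.
; Player overlap with the detect area only prints the character's name, and construction doubles the mesh scale.
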(event `self.ReceiveBeginPlay`
  (`self.Moving`))

(event `Moving`
  (`TimelineComponent.SetPlayRate` (`self.MoveRock`) (/ 1.0 (`self.durantion`)))
  (`TimelineComponent.SetNewTime` (`self.MoveRock`) (`self.rockStartOffset`))
  (bind (_direction _alpha) (`Timeline|MoveRock`)
    (:`Update`
      (set `self.alpha` _alpha)
      (`self.K2_SetActorLocationAndRotation` (`SplineComponent.GetLocationAtDistanceAlongSpline` (`/Game/Prog/blueprint/Traps/Track.Spline` (`self.trackRef`)) (`KismetMathLibrary.Lerp` 0.0 (`SplineComponent.GetSplineLength` (`/Game/Prog/blueprint/Traps/Track.Spline` (`self.trackRef`))) (`self.alpha`)) "World")))))

(event `self.playerDetectArea.OnComponentBeginOverlap`
  (params (OverlappedComponent :type "PrimitiveComponent Object Reference") (OtherActor :type "Actor Object Reference") (OtherComp :type "PrimitiveComponent Object Reference") (OtherBodyIndex :type Integer) (bFromSweep :type Boolean) (SweepResult :type "HitResult Structure (by ref)"))
  (bind _astop_down_character (cast `/Game/Prog/topDownBear/Blueprints/TopDownCharacter` OtherActor))
  (`KismetSystemLibrary.PrintString` (`KismetSystemLibrary.GetDisplayName` _astop_down_character)))

(fn `UserConstructionScript`
  (`parent.UserConstructionScript`)
  (`SceneComponent.SetWorldScale3D` (`self.StaticMesh`) (2.0 2.0 2.0)))