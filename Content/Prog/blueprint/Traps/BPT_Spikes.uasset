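; BPT_Spikes is a spike trap that springs shortly after the player enters its detect area.
; A timeline rotates the mesh's roll, pauses, deactivates the trap and reverses, then re-arms the DoOnce gate.
; While active, Tick calls the player's damage screen feedback every frame they overlap the mesh.
; DoOnce precedes the character cast, so any overlapping actor consumes the trigger until reset.
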(event `self.playerDetectArea.OnComponentBeginOverlap`
  (params (OverlappedComponent :type "PrimitiveComponent Object Reference") (OtherActor :type "Actor Object Reference") (OtherComp :type "PrimitiveComponent Object Reference") (OtherBodyIndex :type Integer) (bFromSweep :type Boolean) (SweepResult :type "HitResult Structure (by ref)"))
  (`/Engine/EditorBlueprintResources/StandardMacros.DoOnce` false :!label _label
    (:`Completed`
      (cast `/Game/Prog/topDownBear/Blueprints/TopDownCharacter` OtherActor)
      (`KismetSystemLibrary.Delay` 0.5)
      (set `self.Activated` true)
      (`self.TrapAction`))))

(event `ResetTrap`
  (goto _label :!via `Reset`))

(event `self.ReceiveTick`
  (params (DeltaSeconds :type "Float (single-precision)"))
  (if (and (`self.Activated`) (`self.playerOverlapping`))
    (`/Game/Prog/topDownBear/Blueprints/TopDownCharacter.DamageScreenFeedback` (`self.playerRef`))))

(event `self.StaticMesh.OnComponentBeginOverlap`
  (params (OverlappedComponent :type "PrimitiveComponent Object Reference") (OtherActor :type "Actor Object Reference") (OtherComp :type "PrimitiveComponent Object Reference") (OtherBodyIndex :type Integer) (bFromSweep :type Boolean) (SweepResult :type "HitResult Structure (by ref)"))
  (bind _astop_down_character (cast `/Game/Prog/topDownBear/Blueprints/TopDownCharacter` OtherActor))
  (set `self.playerOverlapping` true)
  (set `self.playerRef` _astop_down_character))

(event `self.StaticMesh.OnComponentEndOverlap`
  (params (OverlappedComponent :type "PrimitiveComponent Object Reference") (OtherActor :type "Actor Object Reference") (OtherComp :type "PrimitiveComponent Object Reference") (OtherBodyIndex :type Integer))
  (cast `/Game/Prog/topDownBear/Blueprints/TopDownCharacter` OtherActor)
  (set `self.playerOverlapping` false)
  (set `self.playerRef` null))

(event `TrapAction`
  (bind (_rotator_roll _rotator_pitch _rotator_yaw) (`KismetMathLibrary.BreakRotator` (`self.rotator`)))
  (bind (_direction _rotatescale) (`Timeline|RotateTrap` :!via `PlayFromStart` :!label _label_2)
    (:`Update`
      (`SceneComponent.K2_SetWorldRotation` (`self.StaticMesh`) (`KismetMathLibrary.MakeRotator` (* _rotatescale _rotator_roll) _rotator_pitch _rotator_yaw) false false))
    (:`Finished`
      (if (== _direction (enumliteral `ETimelineDirection` "Backward"))
        (`self.ResetTrap`)
        (else
          (`KismetSystemLibrary.Delay` 2.0)
          (set `self.Activated` false)
          (goto _label_2 :!via `ReverseFromEnd`))))))

(fn `UserConstructionScript`
  (`parent.UserConstructionScript`))