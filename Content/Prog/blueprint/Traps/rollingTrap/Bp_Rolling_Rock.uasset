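; Rolling rock trap that damages the TopDownCharacter it hits, then shatters and disappears.
; On first hit, radius damage breaks its destructible mesh, the character takes damage, a Wwise explosion plays and player input is re-enabled.
; It flags itself finished, updates the game instance, then after a delay a timeline dissolves the debris via a material parameter before destroying the actor.
; AlreadyFinished removes the rock immediately.
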(event `self.ReceiveHit`
  (params (MyComp :type "PrimitiveComponent Object Reference") (Other :type "Actor Object Reference") (OtherComp :type "PrimitiveComponent Object Reference") (bSelfMoved :type Boolean) (HitLocation :type "Vector Structure") (HitNormal :type "Vector Structure") (NormalImpulse :type "Vector Structure") (Hit :type "HitResult Structure (by ref)"))
  (bind _destructible (`self.Destructible`))
  (bind _astop_down_character (cast `/Game/Prog/topDownBear/Blueprints/TopDownCharacter` Other))
  (`/Engine/EditorBlueprintResources/StandardMacros.DoOnce` false
    (:`Completed`
      (`DestructibleComponent.ApplyRadiusDamage` _destructible 5000.0 (`SceneComponent.K2_GetComponentLocation` _destructible) 5000.0 5000.0 true)
      (`/Game/Prog/topDownBear/Blueprints/TopDownCharacter.getDamaged` _astop_down_character (`self.Degats`))
      (`AkGameplayStatics.PostEvent` "/Game/sound_design/Wwise/Traps/E_Traps_BigRockExplode.E_Traps_BigRockExplode" (`GameplayStatics.GetPlayerController` 0))
      (set `/Game/Prog/topDownBear/Blueprints/TopDownCharacter.addScreen` false _astop_down_character)
      (`self.EnableInput` _astop_down_character (`GameplayStatics.GetPlayerController` 0))
      (set `self.?Finished` true)
      (`self.UpdateGameInstance`)
      (`KismetSystemLibrary.Delay` 3.0)
      (bind (_direction _time_to_disolve) (`Timeline|Timeline_0`)
        (:`Update`
          (`MeshComponent.SetScalarParameterValueOnMaterials` (`self.Destructible`) "Amount" _time_to_disolve))
        (:`Finished`
          (`self.K2_DestroyActor`))))))

(event `self.AlreadyFinished`
  (`self.K2_DestroyActor`))

(fn `UserConstructionScript`)