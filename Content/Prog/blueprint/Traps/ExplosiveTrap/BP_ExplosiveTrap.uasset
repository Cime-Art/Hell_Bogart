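; Tripwire trap actor with two explosives linked by a cable, which detonates when a TopDownCharacter crosses it.
; The construction script and BeginPlay size the trigger capsule from the distance between the explosives and attach the cable end.
; The first overlap removes the cable after a short delay, waits a configurable fuse time, spawns both explosions and removes the explosives.
; Characters still inside the blast sphere at detonation take damage.
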(event `self.ReceiveBeginPlay`
  (`CapsuleComponent.SetCapsuleHalfHeight` (`self.Capsule`) (/ (`KismetMathLibrary.VSize` (- (`SceneComponent.K2_GetComponentLocation` (`self.Explosive1`)) (`SceneComponent.K2_GetComponentLocation` (`self.Explosive2`)))) 2.0) true)
  (`CableComponent.SetAttachEndToComponent` (`self.CableR`) (`self.Explosive2`) "Explosive2"))

(event `self.Capsule.OnComponentBeginOverlap`
  (params (OverlappedComponent :type "PrimitiveComponent Object Reference") (OtherActor :type "Actor Object Reference") (OtherComp :type "PrimitiveComponent Object Reference") (OtherBodyIndex :type Integer) (bFromSweep :type Boolean) (SweepResult :type "HitResult Structure (by ref)"))
  (bind _explosive1 (`self.Explosive1`))
  (cast `/Game/Prog/topDownBear/Blueprints/TopDownCharacter` OtherActor)
  (`/Engine/EditorBlueprintResources/StandardMacros.DoOnce` false
    (:`Completed`
      (`KismetSystemLibrary.Delay` 0.5)
      (`ActorComponent.K2_DestroyComponent` (`self.CableR`))
      (`KismetSystemLibrary.Delay` (`self.time to explose`))
      (`GameplayStatics.SpawnEmitterAtLocation` "/Game/Graphs/Particles/Grenade/Basic_Grenade/Grenade_Standard.Grenade_Standard" (`SceneComponent.K2_GetComponentLocation` _explosive1))
      (`GameplayStatics.SpawnEmitterAtLocation` "/Game/Graphs/Particles/Grenade/Basic_Grenade/Grenade_Standard.Grenade_Standard" (`SceneComponent.K2_GetComponentLocation` (`self.Explosive2`)))
      (`ActorComponent.K2_DestroyComponent` _explosive1)
      (`ActorComponent.K2_DestroyComponent` (`self.Explosive2`))
      (for _array_element (`PrimitiveComponent.GetOverlappingActors` (`self.Sphere`) "/Game/Prog/topDownBear/Blueprints/TopDownCharacter.TopDownCharacter_C")
        (bind _astop_down_character (cast `/Game/Prog/topDownBear/Blueprints/TopDownCharacter` _array_element))
        (`/Game/Prog/topDownBear/Blueprints/TopDownCharacter.getDamaged` _astop_down_character (`self.Degat`))))))

(fn `UserConstructionScript`
  (`CapsuleComponent.SetCapsuleHalfHeight` (`self.Capsule`) (/ (`KismetMathLibrary.VSize` (- (`SceneComponent.K2_GetComponentLocation` (`self.Explosive1`)) (`SceneComponent.K2_GetComponentLocation` (`self.Explosive2`)))) 2.0) true)
  (`CableComponent.SetAttachEndToComponent` (`self.CableR`) (`self.Explosive2`) "Explosive2"))