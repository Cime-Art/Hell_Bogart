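; Loot chest that opens once, when a TopDownCharacter overlaps its Box.
; Activate plays the Coffre animation, then rolls each ItemsToSpawn entry against its chance and spawns winning BP_Items at LocationSpawnItem, passing itself to their Creation.
; SpawnAgain is an experimental staggered drop using delayed recursion; nothing here starts it, and it halts at the first failed roll.
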(event `SpawnAgain`
  ;[1 1 1] Tests delay entre les spawn
  (bind _keys (`BlueprintMapLibrary.Map_Keys` (`self.itemsToSpawn`)))
  (bind _output (`|GetArrayItem` _keys (`self.dropCount`)))
  (if (<= (`KismetMathLibrary.RandomFloat`) (`BlueprintMapLibrary.Map_Find` (`self.itemsToSpawn`) _output))
    (bind _returnvalue (`|SpawnActorFromClass` "/Game/Prog/blueprint/items/BP_Item.BP_Item_C" (`KismetMathLibrary.MakeTransform` (`SceneComponent.K2_GetComponentLocation` (`self.locationSpawnItem`))) "AdjustIfPossibleButAlwaysSpawn" "OverrideRootScale" null null))
    (set `/Game/Prog/blueprint/items/BP_Item.itemName` _output _returnvalue)
    (`/Game/Prog/blueprint/items/BP_Item.creation` _returnvalue self)
    (`/Engine/EditorBlueprintResources/StandardMacros.IncrementInt` (`self.dropCount`)
      (:`  `
        (if (< (`self.dropCount`) (`BlueprintMapLibrary.Map_Length` (`self.itemsToSpawn`)))
          (`KismetSystemLibrary.Delay` 0.2)
          (`self.SpawnAgain`))))))

(event `Activate`
  (bind _itemstospawn (`self.itemsToSpawn`))
  (`/Engine/EditorBlueprintResources/StandardMacros.DoOnce` false
    (:`Completed`
      (set `self.Open` true)
      (`SkeletalMeshComponent.PlayAnimation` (`self.coffre`) null false)
      ;[1 1 1] DropItems
      (bind _keys (`BlueprintMapLibrary.Map_Keys` _itemstospawn))
      (for _array_element _keys
        (if (<= (`KismetMathLibrary.RandomFloat`) (`BlueprintMapLibrary.Map_Find` _itemstospawn _array_element))
          (bind _returnvalue (`|SpawnActorFromClass` "/Game/Prog/blueprint/items/BP_Item.BP_Item_C" (`KismetMathLibrary.MakeTransform` (`SceneComponent.K2_GetComponentLocation` (`self.locationSpawnItem`)) (struct)) "AdjustIfPossibleButAlwaysSpawn" "OverrideRootScale" null null))
          (set `/Game/Prog/blueprint/items/BP_Item.itemName` _array_element _returnvalue)
          (`/Game/Prog/blueprint/items/BP_Item.creation` _returnvalue self))))))

(event `self.Box.OnComponentBeginOverlap`
  (params (OverlappedComponent :type "PrimitiveComponent Object Reference") (OtherActor :type "Actor Object Reference") (OtherComp :type "PrimitiveComponent Object Reference") (OtherBodyIndex :type Integer) (bFromSweep :type Boolean) (SweepResult :type "HitResult Structure (by ref)"))
  ;[1 1 1] A modif pour interaction avec player
  (cast `/Game/Prog/topDownBear/Blueprints/TopDownCharacter` OtherActor)
  (`self.Activate`))

(fn `UserConstructionScript`)