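; Game instance that keeps event progress and player stats, handles save, load and reset, and drives Wwise jungle music.
; SetEvents registers each map's EVENT actors by display name or re-applies their finished state, and UpdateEvents writes changes back to EVENTS.
; SaveGame stores map, events and stats to a slot, while LoadGame only retrieves the save object.
; PlayMusicJungle feeds closest-enemy distance to an RTPC and switches Exploration/Fight states.
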(fn `EventToString`
  (params (Event :type "/Game/Prog/mapEnigme/EVENT_SYSTEM/EVENT Object Reference") (`StringToEvent?` :type Boolean) (String :type String))
  (returns (ToEvent :type "/Game/Prog/mapEnigme/EVENT_SYSTEM/EVENT Object Reference") (ToString :type String))
  (locals (localEvent :type "/Game/Prog/mapEnigme/EVENT_SYSTEM/EVENT Object Reference") (localEventName :type String) (localReturnEvent :type "/Game/Prog/mapEnigme/EVENT_SYSTEM/EVENT Object Reference") (`eventFound?` :type Boolean))
  (set `local.localEvent` Event)
  (set `local.localEventName` String)
  (if (not `StringToEvent?`)
    ;[1 1 1] Retourne le DisplayName de l'Event
    (return null (`KismetSystemLibrary.GetDisplayName` (`local.localEvent`)))
    (else
      ;[1 1 1] Cherche l'Event a partir du string fourni si il est trouvé renvoie l'Event.
      (bind _outactors (`GameplayStatics.GetAllActorsOfClass` "/Game/Prog/mapEnigme/EVENT_SYSTEM/EVENT.EVENT_C"))
      (for _array_element _outactors
        (if (`KismetStringLibrary.EqualEqual_StrStr` (`KismetSystemLibrary.GetDisplayName` _array_element) (`local.localEventName`))
          (set `local.localReturnEvent` _array_element)
          (set `local.eventFound?` true)
          (break)))
      (if (`local.eventFound?`)
        (return (`local.localReturnEvent`) "")
        (else
          (return null "EventNotFound"))))))

(fn `LoadGame`
  (bind _returnvalue (`GameplayStatics.LoadGameFromSlot` "UserData"))
  (bind _assave (cast `/Game/Prog/blueprint/Save` _returnvalue))
  (set `self.Save` _assave))

(fn `LogEvents`
  (bind _currentevents (`self.currentEvents`))
  (bind _keys (`BlueprintMapLibrary.Map_Keys` _currentevents))
  (for (_array_element _array_index) _keys
    (`KismetSystemLibrary.PrintString` _array_element false)
    (bind _values (`BlueprintMapLibrary.Map_Values` _currentevents))
    (for (_array_element_2 _array_index_2) _values
      (if (== _array_index_2 _array_index)
        (`KismetSystemLibrary.PrintString` (`KismetStringLibrary.Conv_BoolToString` _array_element_2) false)
        (break)))))

(fn `PlayMusicJungle`
  (params (player :type "/Game/Prog/topDownBear/Blueprints/TopDownCharacter Object Reference"))
  ;[1 1 1] Sound Design
  (if (== (`KismetArrayLibrary.Array_Length` (`/Game/Prog/topDownBear/Blueprints/TopDownCharacter.Enemies` player)) 0)
    (`/Engine/EditorBlueprintResources/StandardMacros.DoOnce` false :!label _label
      (:`Completed`
        (`AkGameplayStatics.SetState` "Music_STATE" "Exploration")))
    (else
      (`|ExecutionSequence`
        (:`then_0`
          (goto _label :!via `Reset`))
        (:`then_1`
          (for (_array_element _array_index) (`/Game/Prog/topDownBear/Blueprints/TopDownCharacter.Enemies` player)
            (if (== _array_index 0)
              (bind _returnvalue (`Actor.GetDistanceTo` player _array_element))
              (set `/Game/Prog/topDownBear/Blueprints/TopDownCharacter.closestEnemy` _returnvalue player)
              (elif (< _returnvalue (`/Game/Prog/topDownBear/Blueprints/TopDownCharacter.closestEnemy` player))
                (set `/Game/Prog/topDownBear/Blueprints/TopDownCharacter.closestEnemy` _returnvalue player))))
          (`|ExecutionSequence`
            (:`then_0`
              (`AkGameplayStatics.SetRTPCValue` "Mus_Jungle_Distance_From_Enemy_GP" (`/Game/Prog/topDownBear/Blueprints/TopDownCharacter.closestEnemy` player)))
            (:`then_1`
              (if (<= (`/Game/Prog/topDownBear/Blueprints/TopDownCharacter.closestEnemy` player) 1000.0)
                (`AkGameplayStatics.SetState` "Music_STATE" "Fight")
                (else
                  (`AkGameplayStatics.SetState` "Music_STATE" "Exploration"))))))))))

(fn `ResetGameInstance`
  (set `self.playerStats` (struct))
  (set `self.launchGame` false)
  (`KismetArrayLibrary.Array_Clear` (`self.EVENTS`))
  (`BlueprintMapLibrary.Map_Clear` (`self.currentEvents`)))

(fn `SaveGame`
  (bind _save (`self.Save`))
  (`/Engine/EditorBlueprintResources/StandardMacros.IsValid` (`self.Save`)
    (:`Is Valid`
      (bind _returnvalue (`GameplayStatics.CreateSaveGameObject` "/Game/Prog/blueprint/Save.Save_C"))
      (set `self.Save` _returnvalue))
    (:`Is Not Valid`
      _))
  (set `/Game/Prog/blueprint/Save.currentMap` (`/Game/Prog/topDownBear/Blueprints/TopDownCharacter.currentMap` (cast `/Game/Prog/topDownBear/Blueprints/TopDownCharacter` (`GameplayStatics.GetPlayerPawn` 0) :!pure true)) _save)
  (set `/Game/Prog/blueprint/Save.events` (`self.EVENTS`) _save)
  (set `/Game/Prog/blueprint/Save.playerStats` (`self.playerStats`) _save)
  (`GameplayStatics.SaveGameToSlot` _save (`/Game/Prog/blueprint/Save.UserData` _returnvalue) (`/Game/Prog/blueprint/Save.UserIndex` _returnvalue)))

(fn `SetEvents`
  (locals (`?found` :type Boolean))
  (`BlueprintMapLibrary.Map_Clear` (`self.currentEvents`))
  (for _array_element (`self.EVENTS`)
    (if (== (break `/Game/Prog/mapEnigme/EVENT_SYSTEM/Struct_Events` _array_element) (`/Game/Prog/topDownBear/Blueprints/TopDownCharacter.currentMap` (`self.GetPlayer`)))
      (set `local.?found` true)
      (set `self.currentEvents` (`.EventsName_Finished?_12_6746FBD24EA3BB848AF87BB3487C1FB3` (break `/Game/Prog/mapEnigme/EVENT_SYSTEM/Struct_Events` _array_element)))
      (break)))
  (if (`local.?found`)
    ;[1 1 1] Pour chaque Event sur la map déja enregistrés, si le booléen est vrai  set son booléen '?Finished' a True et appelle la fonction 'AlreadyFinished' de l'Event
    (bind _keys (`BlueprintMapLibrary.Map_Keys` (`self.currentEvents`)))
    (for (_array_element_2 _array_index) _keys
      (bind _values (`BlueprintMapLibrary.Map_Values` (`self.currentEvents`)))
      (if (`|GetArrayItem` _values _array_index)
        (bind _toevent (`self.EventToString` null true _array_element_2))
        (set `/Game/Prog/mapEnigme/EVENT_SYSTEM/EVENT.?Finished` true _toevent)
        (`/Game/Prog/mapEnigme/EVENT_SYSTEM/EVENT.AlreadyFinished` _toevent)))
    (else
      ;[1 1 1] Ajout des event de la map dans EVENTS pour la première fois
      (bind _outactors (`GameplayStatics.GetAllActorsOfClass` "/Game/Prog/mapEnigme/EVENT_SYSTEM/EVENT.EVENT_C"))
      (for _array_element_3 _outactors
        (bind (_toevent_2 _tostring) (`self.EventToString` _array_element_3))
        (`BlueprintMapLibrary.Map_Add` (`self.currentEvents`) _tostring))
      (if (> (`BlueprintMapLibrary.Map_Length` (`self.currentEvents`)) 0)
        (`KismetArrayLibrary.Array_AddUnique` (`self.EVENTS`) (make `/Game/Prog/mapEnigme/EVENT_SYSTEM/Struct_Events` (`self.GetCurrentMap`) (`self.currentEvents`)))))))

(fn `SetMusicjungle`
  (params (player :type "/Game/Prog/topDownBear/Blueprints/TopDownCharacter Object Reference"))
  (`AkGameplayStatics.PostEvent` "/Game/sound_design/Wwise/Music/Jungle/E_Mus_Jungle_Main_Play.E_Mus_Jungle_Main_Play" player))

(fn `UpdateEvents`
  (params (EventToUpdate :type "/Game/Prog/mapEnigme/EVENT_SYSTEM/EVENT Object Reference"))
  (locals (localEvent :type "/Game/Prog/mapEnigme/EVENT_SYSTEM/EVENT Object Reference"))
  (bind _localevent (`local.localEvent`))
  (bind _returnvalue (`KismetSystemLibrary.GetDisplayName` _localevent))
  (set `local.localEvent` EventToUpdate)
  (bind _keys (`BlueprintMapLibrary.Map_Keys` (`self.currentEvents`)))
  (for _array_element _keys
    (if (`KismetStringLibrary.EqualEqual_StrStr` _array_element _returnvalue)
      (`BlueprintMapLibrary.Map_Add` (`self.currentEvents`) _returnvalue (`/Game/Prog/mapEnigme/EVENT_SYSTEM/EVENT.?Finished` _localevent))
      (break)))
  (for (_array_element_2 _array_index) (`self.EVENTS`)
    (if (== (break `/Game/Prog/mapEnigme/EVENT_SYSTEM/Struct_Events` _array_element_2) (`self.GetCurrentMap`))
      (`KismetArrayLibrary.Array_Set` (`self.EVENTS`) _array_index (make `/Game/Prog/mapEnigme/EVENT_SYSTEM/Struct_Events` (break `/Game/Prog/mapEnigme/EVENT_SYSTEM/Struct_Events` _array_element_2) (`self.currentEvents`)))
      (break)))
  (`self.LogEvents`))