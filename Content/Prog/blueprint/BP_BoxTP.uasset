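; BP_BoxTP is a tagged trigger box that starts a black-screen transition for the TopDownCharacter, likely a teleport.
; Overlapping CollisionComponent while GatlingOn is false calls the character's SaveStats, then AddBlackScreen with Tag as the name.
; A second volume, BackWindos, toggles the character's AddScreen flag on begin and end overlap.
; The construction script displays Tag on TextRender and scales BackWindos by AddBlackBar.
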(event `self.CollisionComponent.OnComponentBeginOverlap`
  (params (OverlappedComponent :type "PrimitiveComponent Object Reference") (OtherActor :type "Actor Object Reference") (OtherComp :type "PrimitiveComponent Object Reference") (OtherBodyIndex :type Integer) (bFromSweep :type Boolean) (SweepResult :type "HitResult Structure (by ref)"))
  (bind _astop_down_character (cast `/Game/Prog/topDownBear/Blueprints/TopDownCharacter` OtherActor))
  (if (not (`/Game/Prog/topDownBear/Blueprints/TopDownCharacter.gatlingOn` _astop_down_character))
    (`/Game/Prog/topDownBear/Blueprints/TopDownCharacter.SaveStats` _astop_down_character false)
    (`/Game/Prog/topDownBear/Blueprints/TopDownCharacter.addBlackScreen` _astop_down_character (`KismetStringLibrary.Conv_StringToName` (`self.Tag`)))))

(event `self.backWindos.OnComponentBeginOverlap`
  (params (OverlappedComponent :type "PrimitiveComponent Object Reference") (OtherActor :type "Actor Object Reference") (OtherComp :type "PrimitiveComponent Object Reference") (OtherBodyIndex :type Integer) (bFromSweep :type Boolean) (SweepResult :type "HitResult Structure (by ref)"))
  (bind _astop_down_character (cast `/Game/Prog/topDownBear/Blueprints/TopDownCharacter` OtherActor))
  (set `/Game/Prog/topDownBear/Blueprints/TopDownCharacter.addScreen` true _astop_down_character))

(event `self.backWindos.OnComponentEndOverlap`
  (params (OverlappedComponent :type "PrimitiveComponent Object Reference") (OtherActor :type "Actor Object Reference") (OtherComp :type "PrimitiveComponent Object Reference") (OtherBodyIndex :type Integer))
  (bind _astop_down_character (cast `/Game/Prog/topDownBear/Blueprints/TopDownCharacter` OtherActor))
  (set `/Game/Prog/topDownBear/Blueprints/TopDownCharacter.addScreen` false _astop_down_character))

(fn `UserConstructionScript`
  (`TextRenderComponent.K2_SetText` (`self.TextRender`) (`KismetTextLibrary.Conv_StringToText` (`self.Tag`)))
  (`SceneComponent.SetWorldScale3D` (`self.backWindos`) (`self.addBlackBar`)))