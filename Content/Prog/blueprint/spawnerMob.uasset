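; Mob spawner actor that populates an area with a mix of mob types once, on BeginPlay, if it is activated.
; A random total between the min and max is split by the per-class ratio map, truncating each share.
; Each mob gets a random reachable navmesh point within the spawn radius and a random yaw, and is skipped if collision can't be resolved.
; The construction script sizes the SpawnZone sphere to that radius.
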(event `self.ReceiveBeginPlay`
  (`self.Spawn`))

(fn `Spawn`
  (bind _mobtypes_ratio (`self.mobTypes-ratio`))
  (if (`self.activated`)
    (set `self.MobToSpawn` (`KismetMathLibrary.RandomIntegerInRange` (`self.minMobsToSpawn`) (`self.maxMobsToSpawn`)))
    (bind _keys (`BlueprintMapLibrary.Map_Keys` _mobtypes_ratio))
    (for _array_element _keys
      (for _ (range 1 (+ (`KismetMathLibrary.FTrunc` (* (`self.MobToSpawn`) (`BlueprintMapLibrary.Map_Find` _mobtypes_ratio _array_element))) 1))
        (`|SpawnActorFromClass` _array_element (`KismetMathLibrary.MakeTransform` (`NavigationSystemV1.K2_GetRandomReachablePointInRadius` (`self.K2_GetActorLocation`) (`self.radiusSpawn`) null null) (`KismetMathLibrary.MakeRotator` 0.0 0.0 (`KismetMathLibrary.RandomFloatInRange` 0.0 360.0))) "AdjustIfPossibleButDontSpawnIfColliding" "OverrideRootScale" null null)))))

(fn `UserConstructionScript`
  (`SphereComponent.SetSphereRadius` (`self.spawnZone`) (`self.radiusSpawn`) true))