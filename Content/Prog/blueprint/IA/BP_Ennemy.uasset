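; Enemy character for a top-down game that takes damage, suffers status effects and rewards the player on death.
; GetDamage rolls an instant-kill execution chance or subtracts HP, then ragdolls the dead enemy with an impulse from the explosive shot, grenade or player shot.
; Tick runs burn damage and stun timers, while Slow cuts walk speed.
; Both death paths call DropXpDestroy, which grants XP, rolls loot spawns and destroys the actor after a delay.
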(event `self.ReceiveBeginPlay`
  (set `CharacterMovementComponent.MaxWalkSpeed` (`self.defaultWalkSpeed`) (`self.CharacterMovement`))
  (set `self.player` (cast `/Game/Prog/topDownBear/Blueprints/TopDownCharacter` (`GameplayStatics.GetPlayerCharacter` 0) :!pure true)))

(event `GetDamage`
  (params (Damage :type Integer) (tirExplo :type "/Game/Prog/blueprint/Bp_TirExplo Object Reference") (Grenade :type "/Game/Prog/blueprint/Grenades/BP_Grenade Object Reference") (`Shot Power` :type "Float (double-precision)") (impactNormal :type "Vector Structure"))
  (bind _returnvalue (`self.K2_GetActorLocation`))
  (bind _returnvalue_2 (`self.K2_GetActorLocation` tirExplo))
  (bind _returnvalue_3 (`self.K2_GetActorLocation` Grenade))
  (bind _returnvalue_4 (`self.K2_GetActorLocation`))
  (bind _returnvalue_5 (`self.K2_GetActorLocation`))
  (bind _mesh (`self.Mesh`))
  (bind _mesh_2 (`self.Mesh`))
  (bind _returnvalue_6 (`self.K2_GetActorLocation` (`self.player`)))
  ;[1 0.2 0.2] GetDamage
  ;;[1 1 1] Exec
  (if (> (`KismetMathLibrary.RandomIntegerInRange` 0 100) (- 100 (`self.chanceExec`)))
    (set `self.HP` 0)
    (`GameplayStatics.SpawnEmitterAtLocation` "/Game/Prog/VFX_Grenades/P_Explo_Feu.P_Explo_Feu" (`self.K2_GetActorLocation`) (struct))
    (set `self.isDead` true :!label _label)
    (`/Engine/EditorBlueprintResources/StandardMacros.DoOnce` false
      (:`Completed`
        (`PrimitiveComponent.SetSimulatePhysics` _mesh true)
        (`PrimitiveComponent.SetCollisionProfileName` _mesh "Ragdoll")
        (`PrimitiveComponent.SetCollisionProfileName` (`self.CapsuleComponent`) "NoCollision")
        ;;[1 1 1] Tir explo
        (`/Engine/EditorBlueprintResources/StandardMacros.IsValid` tirExplo
          (:`Is Valid`
            (`PrimitiveComponent.AddImpulse` (`self.Mesh`) (* (`KismetMathLibrary.GetDirectionUnitVector` _returnvalue_2 _returnvalue) (* (- 1.0 (/ (`KismetMathLibrary.Vector_Distance` _returnvalue_2 _returnvalue) (`/Game/Prog/blueprint/Bp_TirExplo.sphereRadius` tirExplo))) `Shot Power`)) "None" false))
          (:`Is Not Valid`
            ;;[1 1 1] Grenade
            (`/Engine/EditorBlueprintResources/StandardMacros.IsValid` Grenade
              (:`Is Valid`
                (`PrimitiveComponent.AddImpulse` (`self.Mesh`) (* (`KismetMathLibrary.GetDirectionUnitVector` _returnvalue_3 _returnvalue_4) (* (- 1.0 (/ (`KismetMathLibrary.Vector_Distance` _returnvalue_3 _returnvalue_4) (`/Game/Prog/blueprint/Grenades/BP_Grenade.radiusExplo` Grenade))) `Shot Power`)) "None" false))
              (:`Is Not Valid`
                (if (== impactNormal (0.0 0.0 0.0))
                  (`PrimitiveComponent.AddImpulse` _mesh_2 (* (`KismetMathLibrary.GetDirectionUnitVector` _returnvalue_6 _returnvalue_5) (* (- 1.0 (/ (`KismetMathLibrary.Vector_Distance` _returnvalue_6 _returnvalue_5) (`/Game/Prog/topDownBear/Blueprints/TopDownCharacter.distanceShot` (`self.player`)))) `Shot Power`)) "None" false)
                  (else
                    (`PrimitiveComponent.AddImpulse` _mesh_2 (* (* impactNormal (* (`KismetMathLibrary.GetDirectionUnitVector` (`self.K2_GetActorLocation` (`self.player`)) (`self.K2_GetActorLocation`)) -1.0)) (/ `Shot Power` 1.0)) "None" false)))))))
        (`self.Drop/Xp/Destroy`)))
    (else
      (set `self.HP` (- (`self.HP`) Damage))
      (if (<= (`self.HP`) 0)
        (goto _label)
        (else
          (set `self.takeDamag?` true))))))

(event `self.ReceiveTick`
  (params (DeltaSeconds :type "Float (single-precision)"))
  (bind _mesh (`self.Mesh`))
  (`|ExecutionSequence`
    (:`then_1`
      ;[30 0 30] Fire / Stun (a modifier)
      (if (`self.burning`)
        (bind _output_get (set `self.timerBurning` (+ DeltaSeconds (`self.timerBurning`))))
        (if (> _output_get 0.5)
          (set `self.burnLifeTime` (- (`self.burnLifeTime`) 1))
          (set `self.timerBurning` 0.0)
          (set `self.HP` (- (`self.HP`) (`self.FireDmg`)))
          (if (and (<= (`self.HP`) 0) (not (`self.isDead`)))
            (set `self.isDead` true)
            (`PrimitiveComponent.SetSimulatePhysics` _mesh true)
            (`PrimitiveComponent.SetCollisionProfileName` _mesh "Ragdoll")
            (`PrimitiveComponent.SetCollisionProfileName` (`self.CapsuleComponent`) "NoCollision")
            (`ActorComponent.Deactivate` (`self.P_Smoke`))
            (`/Engine/EditorBlueprintResources/StandardMacros.DoOnce` false
              (:`Completed`
                (`self.Drop/Xp/Destroy`)))
            (else
              (`|ExecutionSequence`
                (:`then_0`
                  (if (<= (`self.poisonLifeTime`) 0)
                    (set `self.poison` false)
                    (`ActorComponent.Deactivate` (`self.P_Smoke`))))
                (:`then_1`
                  (if (<= (`self.burnLifeTime`) 0)
                    (set `self.burning` false)))))))))
    (:`then_2`
      (if (`self.Stunned`)
        (bind _output_get_2 (set `self.timerStun` (+ DeltaSeconds (`self.timerStun`))))
        (if (>= _output_get_2 (`self.stunTime`))
          (set `self.Stunned` false)
          (set `self.timerStun` 0.0))))))

(event `getDamagesGrenade`
  (params (`Shot Power` :type "Float (double-precision)") (grenade :type "/Game/Prog/blueprint/Grenades/BP_Grenade Object Reference"))
  ;[0 0 0 0 750] Not Used
)

(fn `slow`
  (params (`On/Off` :type Boolean))
  (bind _charactermovement (`self.CharacterMovement`))
  (if `On/Off`
    (set `CharacterMovementComponent.MaxWalkSpeed` (/ (`self.defaultWalkSpeed`) 6.0) _charactermovement)
    (else
      (set `CharacterMovementComponent.MaxWalkSpeed` (`self.defaultWalkSpeed`) _charactermovement))))

(fn `UserConstructionScript`)