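; Enemy character Blueprint for a top-down game, handling damage, elemental status effects, movement locks and death rewards.
; GetDamage applies hits or a random execution; burn and thunder tick through recursive delayed events, while ice slows or freezes via retriggerable delays.
; The death function ragdolls the mesh with a distance-scaled impulse, grants XP and spawns randomly named loot by type and rarity.
; SpawnDissolve and Dissolve are empty hooks, and attack, stun and hit reactions mainly set state flags.
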(event `self.ReceiveBeginPlay`
  (set `self.player` (cast `/Game/Prog/topDownBear/Blueprints/TopDownCharacter` (`GameplayStatics.GetPlayerCharacter` 0) :!pure true))
  (if (`self.?spawnParticle`)
    (`self.SpawnDissolve`)))

(event `SpawnDissolve`)

(event `Dissolve`)

(event `GetDamage`
  (params (Damage :type Integer) (Grenade :type "/Game/Prog/blueprint/Grenades/BP_Grenade Object Reference") (impactNormal :type "Vector Structure") (TickingDamage :type Boolean))
  ;[1 0.2 0.2] GetDamage
  (if (and (not (`KismetSystemLibrary.IsValid` Grenade)) (not TickingDamage) (> (`KismetMathLibrary.RandomIntegerInRange` 0 100) (- 100 (`self.chanceExec`))))
    ;;[1 1 1] Effet execution (temp)
    (set `self.HP` 0)
    (`GameplayStatics.SpawnEmitterAtLocation` "/Game/Prog/VFX_Grenades/P_Explo_Feu.P_Explo_Feu" (`self.K2_GetActorLocation`) (struct) (0.25 0.25 0.25))
    (`ActorComponent.Deactivate` (`self.P_Fire`) :!label _label)
    (else
      (set `self.HP` (- (`self.HP`) Damage))
      (if (<= (`self.HP`) 0)
        (goto _label)
        (else
          (`self.TakingDamage` TickingDamage))))))

(event `TurnFreezed`
  (params (freezeTime :type "Float (double-precision)"))
  (bind _mesh (`self.Mesh`))
  ;[1 1 1] Ice Grenade Effect
  (if (`self.Freezed?`)
    (`KismetSystemLibrary.PrintString` "freeze")
    (else
      (`AkGameplayStatics.PostEvent` "/Game/sound_design/Wwise/Enemis/MobJungleCharlie/E_DotElement_Ice_Begin.E_DotElement_Ice_Begin" self)))
  (set `self.Freezed?` true)
  (`self.Freeze Mat`)
  (`self.CanMove` false)
  (set `SkeletalMeshComponent.bPauseAnims` true _mesh)
  (`KismetSystemLibrary.RetriggerableDelay` freezeTime)
  (if (not (`self.isDead`))
    (set `SkeletalMeshComponent.bPauseAnims` false _mesh)
    (set `self.Freezed?` false)
    (`self.Freeze Mat`)
    (`AkGameplayStatics.PostEvent` "/Game/sound_design/Wwise/Enemis/MobJungleCharlie/E_DotElement_Ice_End.E_DotElement_Ice_End" self)
    (`ActorComponent.Deactivate` (`self.ice02`))
    (if (not (`self.Attacking?`))
      (`self.CanMove` true true)
      (`ActorComponent.Deactivate` (`self.ice`)))))

(event `TurnSlow`
  (params (SlowTime :type "Float (double-precision)"))
  ;[1 1 1] Ice ammo effect
  (if (not (`self.slow?`))
    (`AkGameplayStatics.PostEvent` "/Game/sound_design/Wwise/Enemis/MobJungleCharlie/E_DotElement_Ice_Begin.E_DotElement_Ice_Begin" self))
  (set `CharacterMovementComponent.MaxWalkSpeed` (/ (`self.defaultWalkSpeed`) 2.0) (`self.CharacterMovement`))
  (set `self.slow?` true)
  (`ActorComponent.Activate` (`self.ice02`) false)
  (`KismetSystemLibrary.RetriggerableDelay` SlowTime)
  (set `CharacterMovementComponent.MaxWalkSpeed` (`self.defaultWalkSpeed`) (`self.CharacterMovement`))
  (set `self.slow?` false)
  (`ActorComponent.Deactivate` (`self.ice02`))
  (`AkGameplayStatics.PostEvent` "/Game/sound_design/Wwise/Enemis/MobJungleCharlie/E_DotElement_Ice_End.E_DotElement_Ice_End" self))

(event `Freeze Mat`
  (bind _mesh (`self.Mesh`))
  (bind _mesh_2 (`self.Mesh`))
  ;[1 1 1] Set Freeze Materials
  (if (`self.Freezed?`)
    (`PrimitiveComponent.SetMaterial` _mesh 0 "/Game/Graphs/Particles/Dotparticules/Mat_DotIce_Inst_JC.Mat_DotIce_Inst_JC")
    (`PrimitiveComponent.SetMaterial` _mesh 1 "/Game/Graphs/Particles/Dotparticules/Mat_DotIce_Inst_JC.Mat_DotIce_Inst_JC")
    (`ActorComponent.Activate` (`self.ice02`) false)
    (else
      (`ActorComponent.Activate` (`self.ice`) false)
      (`PrimitiveComponent.SetMaterial` _mesh_2 0 "/Game/Graphs/Test_up/Bones_Disolve_inst.Bones_Disolve_inst")
      (`PrimitiveComponent.SetMaterial` _mesh_2 1 (`self.DefaultMaterial`)))))

(event `TurnBurn`
  (params (nbTick :type Integer) (FireDamage :type Integer))
  ;[1 1 1] Fire Grenade / Ammo Effect
  (if (not (`self.isDead`))
    (if (not (`self.IsBurn`))
      (`AkGameplayStatics.PostEvent` "/Game/sound_design/Wwise/Enemis/MobJungleCharlie/E_DotElement_Fire_Begin.E_DotElement_Fire_Begin" self))
    (set `self.IsBurn` true)
    (`ActorComponent.SetActive` (`self.P_Fire`) true false)
    (if (> nbTick 0)
      (`self.GetDamage` FireDamage null (0.0 0.0 0.0) true)
      (if (and (`self.IsBurn`) (`self.isDead`))
        (`KismetSystemLibrary.Delay` 3.0)
        (else
          (`KismetSystemLibrary.RetriggerableDelay` 0.5)
          (`self.TurnBurn` (- nbTick 1) FireDamage)))
      (else
        (`ActorComponent.Deactivate` (`self.P_Fire`))
        (set `self.IsBurn` false)
        (`AkGameplayStatics.PostEvent` "/Game/sound_design/Wwise/Enemis/MobJungleCharlie/E_DotElement_Fire_End.E_DotElement_Fire_End" self)))))

(event `Thunder`
  (params (`Nb Tick` :type Integer) (`electric damage` :type Integer) (`slow time` :type "Float (double-precision)"))
  ;[1 1 1] Thunder grenade / Ammo effect
  (if (not (`self.isDead`))
    (if (not (`self.slow?`))
      (`AkGameplayStatics.PostEvent` "/Game/sound_design/Wwise/Enemis/MobJungleCharlie/E_DotElement_Thunder_Begin.E_DotElement_Thunder_Begin" self))
    (`|ExecutionSequence`
      (:`then_0`
        (`ActorComponent.SetActive` (`self.stun`) true false)
        (`ActorComponent.SetActive` (`self.Electric`) true false)
        (if (> `Nb Tick` 0)
          (`self.GetDamage` `electric damage` null (0.0 0.0 0.0) true)
          (`KismetSystemLibrary.RetriggerableDelay` 0.5)
          (`self.Thunder` (- `Nb Tick` 1) `electric damage`)
          (else
            (`ActorComponent.Deactivate` (`self.stun`))
            (`ActorComponent.Deactivate` (`self.Electric`)))))
      (:`then_1`
        (set `CharacterMovementComponent.MaxWalkSpeed` (/ (`self.defaultWalkSpeed`) 2.0) (`self.CharacterMovement`))
        (set `self.slow?` true)
        (`KismetSystemLibrary.RetriggerableDelay` `slow time`)
        (set `CharacterMovementComponent.MaxWalkSpeed` (`self.defaultWalkSpeed`) (`self.CharacterMovement`))
        (set `self.slow?` false)
        (`AkGameplayStatics.PostEvent` "/Game/sound_design/Wwise/Enemis/MobJungleCharlie/E_DotElement_Thunder_End.E_DotElement_Thunder_End" self)))
    (else
      (`KismetSystemLibrary.Delay` 0.5)
      (`ActorComponent.Deactivate` (`self.stun`))
      (`ActorComponent.Deactivate` (`self.Electric`)))))

(event `TurnStun`
  (`self.CanMove` false)
  (set `self.Stunned?` true))

(event `StartAttack`
  (params (`distanceAttack?` :type Boolean))
  (if (not (`self.Attacking?`))
    (`self.CanMove` false true)
    (set `self.distanceAttack?` `distanceAttack?`)
    (set `self.Attacking?` true)
    (set `self.PlayerHit?` false)))

(event `TakingDamage`
  (params (`tickingDamage?` :type Boolean))
  (if (!= (`self.TypeEnemy`) 3)
    (if (not (or `tickingDamage?` (`self.Freezed?`) (`self.Stunned?`)))
      (`self.CanMove` false)
      (set `self.Damaged?` true))))

(event `CanMove`
  (params (`canMove?` :type Boolean) (`canRotate?` :type Boolean))
  (bind _charactermovement (`self.CharacterMovement`))
  (if `canMove?`
    (`CharacterMovementComponent.SetMovementMode` _charactermovement "MOVE_Walking" 0)
    (elif `canRotate?`
      (`CharacterMovementComponent.SetMovementMode` _charactermovement "MOVE_Custom" 0)
      (else
        (`CharacterMovementComponent.DisableMovement` _charactermovement)))))

(fn `CheckLootPriority`
  (returns (LC :type "Float (double-precision)") (LR :type String) (MC :type "Float (double-precision)") (MR :type String) (BG :type "Float (double-precision)") (BR :type String))
  (locals (BiggerChance :type "Float (double-precision)") (MidChance :type "Float (double-precision)") (LowerChance :type "Float (double-precision)") (BiggerRarity :type String) (MidRarity :type String) (LowerRarity :type String))
  (bind _chancestandard (`self.chanceStandard`))
  (bind _chanceepic (`self.chanceEpic`))
  (bind _chancelegendary (`self.ChanceLegendary`))
  (bind _chanceepic_2 (`self.chanceEpic`))
  (bind _chancelegendary_2 (`self.ChanceLegendary`))
  (bind _chancestandard_2 (`self.chanceStandard`))
  (bind _chanceepic_3 (`self.chanceEpic`))
  (bind _chancestandard_3 (`self.chanceStandard`))
  (bind _chancelegendary_3 (`self.ChanceLegendary`))
  (if (and (> _chancestandard (`self.chanceEpic`)) (> _chancestandard (`self.ChanceLegendary`)))
    (set `local.BiggerChance` (`self.chanceStandard`))
    (set `local.BiggerRarity` "01")
    (if (> (`self.chanceEpic`) (`self.ChanceLegendary`))
      (set `local.MidChance` _chanceepic)
      (set `local.MidRarity` "02")
      (set `local.LowerChance` _chancelegendary)
      (set `local.LowerRarity` "03")
      (else
        (set `local.MidChance` _chancelegendary)
        (set `local.MidRarity` "03")
        (set `local.LowerChance` _chanceepic)
        (set `local.LowerRarity` "02")))
    (return (`local.LowerChance`) (`local.LowerRarity`) (`local.MidChance`) (`local.MidRarity`) (`local.BiggerChance`) (`local.BiggerRarity`))
    (elif (and (> _chancelegendary_2 (`self.chanceStandard`)) (> _chancelegendary_2 (`self.chanceEpic`)))
      (set `local.BiggerChance` (`self.ChanceLegendary`))
      (set `local.BiggerRarity` "03")
      (if (> (`self.chanceStandard`) (`self.chanceEpic`))
        (set `local.MidChance` _chancestandard_3)
        (set `local.MidRarity` "01")
        (set `local.LowerChance` _chanceepic_3)
        (set `local.LowerRarity` "02")
        (else
          (set `local.MidChance` _chanceepic_3)
          (set `local.MidRarity` "02")
          (set `local.LowerChance` _chancestandard_3)
          (set `local.LowerRarity` "01")))
      (return (`local.LowerChance`) (`local.LowerRarity`) (`local.MidChance`) (`local.MidRarity`) (`local.BiggerChance`) (`local.BiggerRarity`))
      (elif (and (> _chanceepic_2 (`self.chanceStandard`)) (> _chanceepic_2 (`self.ChanceLegendary`)))
        (set `local.BiggerChance` (`self.chanceEpic`))
        (set `local.BiggerRarity` "02")
        (if (> (`self.chanceStandard`) (`self.ChanceLegendary`))
          (set `local.MidChance` _chancestandard_2)
          (set `local.MidRarity` "01")
          (set `local.LowerChance` _chancelegendary_3)
          (set `local.LowerRarity` "03")
          (else
            (set `local.MidChance` _chancelegendary_3)
            (set `local.MidRarity` "03")
            (set `local.LowerChance` _chancestandard_2)
            (set `local.LowerRarity` "01")))
        (return (`local.LowerChance`) (`local.LowerRarity`) (`local.MidChance`) (`local.MidRarity`) (`local.BiggerChance`) (`local.BiggerRarity`))))))

(fn `Drop`
  (locals (localRollForRarity :type "Float (double-precision)") (localLC :type "Float (double-precision)" :default 0.0) (localLR :type String) (localMC :type "Float (double-precision)" :default 0.0) (localMR :type String) (localBC :type "Float (double-precision)" :default 0.0) (localBR :type String) (localItemName :type String) (countLoot :type Integer))
  ;[1 1 1] loot?
  (if (> (`self.chanceToLootItems`) (`KismetMathLibrary.RandomFloatInRange` 0.0 99.0)) :!label _label
    ;[1 1 1] Count Loot
    (if (< (`local.countLoot`) (`self.countLootMax`))
      (`/Engine/EditorBlueprintResources/StandardMacros.IncrementInt` (`local.countLoot`)
        (:`  `
          ;[1 1 1] gre/mun
          (switch `int` (`KismetMathLibrary.RandomIntegerInRange` 0 1)
            (:`0`
              ;[1 1 1] type gre
              (set `local.localItemName` (`KismetStringLibrary.Concat_StrStr` (`local.localItemName`) "grenade"))
              (switch `int` (`KismetMathLibrary.RandomIntegerInRange` 0 3)
                (:`0`
                  (set `local.localItemName` (`KismetStringLibrary.Concat_StrStr` (`local.localItemName`) "Fire") :!label _label_2))
                (:`1`
                  (set `local.localItemName` (`KismetStringLibrary.Concat_StrStr` (`local.localItemName`) "Ice") :!label _label_3))
                (:`2`
                  (set `local.localItemName` (`KismetStringLibrary.Concat_StrStr` (`local.localItemName`) "Thunder") :!label _label_4))
                (:`3`
                  (set `local.localItemName` (`KismetStringLibrary.Concat_StrStr` (`local.localItemName`) "Explod")))))
            (:`1`
              ;[1 1 1] type mun
              (set `local.localItemName` (`KismetStringLibrary.Concat_StrStr` (`local.localItemName`) "munition"))
              (switch `int` (`KismetMathLibrary.RandomIntegerInRange` 0 2)
                (:`0`
                  (goto _label_2))
                (:`1`
                  (goto _label_3))
                (:`2`
                  (goto _label_4)))))
          (bind (_lc _lr _mc _mr _bg _br) (`self.CheckLootPriority`))
          (bind _rarity (`self.RollForRarity` (`KismetMathLibrary.RandomFloatInRange` 0.0 100.0) _lc _lr _mc _mr _bg _br))
          (set `local.localItemName` (`KismetStringLibrary.Concat_StrStr` (`local.localItemName`) _rarity))
          (bind _returnvalue (`|SpawnActorFromClass` "/Game/Prog/blueprint/items/BP_Item.BP_Item_C" (`SceneComponent.K2_GetComponentToWorld` (`self.spawnLoot`)) "Undefined" "OverrideRootScale" null null))
          (set `/Game/Prog/blueprint/items/BP_Item.itemName` (`KismetStringLibrary.Conv_StringToName` (`local.localItemName`)) _returnvalue)
          (`/Game/Prog/blueprint/items/BP_Item.creation` _returnvalue 10.0 null)
          (goto _label))))))

(fn `Get_Damage_Death`
  (params (Ref_Grenade :type "/Game/Prog/blueprint/Grenades/BP_Grenade Object Reference"))
  (bind _returnvalue (`self.K2_GetActorLocation`))
  (bind _mesh (`self.Mesh`))
  (bind _returnvalue_2 (`self.K2_GetActorLocation` (select `bool` (`KismetSystemLibrary.IsValid` Ref_Grenade) :`false` (`self.player`) :`true` Ref_Grenade :!type "Actor Object Reference")))
  (set `self.isDead` true)
  (`AkGameplayStatics.PostEvent` "/Game/sound_design/Wwise/Enemis/MobJungleCharlie/E_Mob_JungleCharlie_Death.E_Mob_JungleCharlie_Death" self)
  (`PrimitiveComponent.SetSimulatePhysics` _mesh true)
  (`PrimitiveComponent.SetCollisionProfileName` _mesh "Ragdoll")
  (`PrimitiveComponent.SetCollisionProfileName` (`self.CapsuleComponent`) "NoCollision")
  (`SkeletalMeshComponent.AddImpulseToAllBodiesBelow` (`self.Mesh`) (* (* (`KismetMathLibrary.GetDirectionUnitVector` _returnvalue_2 _returnvalue) (/ 1.0 (`KismetMathLibrary.Vector_Distance2D` _returnvalue_2 _returnvalue))) (`self.ImpulsePower`)) "None" false true)
  (`self.Drop/Xp/Destroy`))

(fn `RollForRarity`
  (params (Roll :type "Float (double-precision)") (LowerChance :type "Float (double-precision)") (lowerRarity :type String) (MidChance :type "Float (double-precision)") (midRarity :type String) (BiggerChance :type "Float (double-precision)") (biggerRarity :type String))
  (returns (Rarity :type String))
  (if (< Roll LowerChance)
    (return lowerRarity)
    (elif (< Roll MidChance)
      (return midRarity)
      (else
        (return biggerRarity)))))

(fn `SetRunningMode`
  (params (`Running?` :type Boolean))
  (bind _defaultwalkspeed (`self.defaultWalkSpeed`))
  (if (not (`self.slow?`))
    (set `CharacterMovementComponent.MaxWalkSpeed` (select `bool` `Running?` :`false` _defaultwalkspeed :`true` (* _defaultwalkspeed 2.0)) (`self.CharacterMovement`))))

(fn `UserConstructionScript`)