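; Boss naginata that is thrown at the player and pulls them back toward IA_Boss.
; On Activate, a timeline lerps the detached mesh from the boss's right wrist to the player's live position, aimed at their spine.
; A second timeline retracts it, dragging the movement-locked player at the lance tip until an event track releases them, then reattaches it.
; The grab always follows the throw without a hit check; older overlap-based logic is unused.
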(event `self.ReceiveBeginPlay`
  (bind _returnvalue (`GameplayStatics.GetActorOfClass` "/Game/Prog/blueprint/IA/IA_Boss.IA_Boss_C"))
  (set `self.boss` _returnvalue))

(event `Activate`
  (bind _returnvalue (`GameplayStatics.GetPlayerCharacter` 0))
  (bind (_returnvalue_x _returnvalue_y _returnvalue_z) (`KismetMathLibrary.BreakVector` (`self.K2_GetActorLocation` _returnvalue)))
  (bind (_returnvalue_x_2 _returnvalue_y_2) (`KismetMathLibrary.BreakVector` (`SceneComponent.GetSocketLocation` (`self.SkeletalMesh`) "JNT_Lance_end")))
  (bind (_returnvalue_roll _returnvalue_pitch _returnvalue_yaw) (`KismetMathLibrary.BreakRotator` (`KismetMathLibrary.FindLookAtRotation` (`SceneComponent.K2_GetComponentLocation` (`self.SkeletalMesh`)) (`SceneComponent.GetSocketLocation` (`Character.Mesh` (`GameplayStatics.GetPlayerCharacter` 0)) "Character1_Spine2"))))
  (`SceneComponent.K2_DetachFromComponent` (`self.SkeletalMesh`) "KeepWorld" "KeepWorld" "KeepWorld" true)
  (set `self.InAir` true)
  (bind (_direction _alpha) (`Timeline|LanceMovement` :!via `PlayFromStart`)
    (:`Update`
      (`SceneComponent.K2_SetWorldLocationAndRotation` (`self.SkeletalMesh`) (`KismetMathLibrary.VLerp` (`SceneComponent.GetSocketLocation` (`Character.Mesh` (`self.boss`)) "JNT_Wrist_R_01Socket") (`self.K2_GetActorLocation` (`GameplayStatics.GetPlayerCharacter` 0)) _alpha) (`KismetMathLibrary.MakeRotator` _returnvalue_roll _returnvalue_pitch (+ _returnvalue_yaw 90.0)) false false))
    (:`Finished`
      (set `self.InAir` false)
      (`PrimitiveComponent.SetCollisionEnabled` (`self.SkeletalMesh`) "NoCollision")
      (`/Game/Prog/topDownBear/Blueprints/TopDownCharacter.CanMove` (cast `/Game/Prog/topDownBear/Blueprints/TopDownCharacter` (`GameplayStatics.GetPlayerCharacter` 0) :!pure true) false true)
      (set `self.GrabLocation` (`SceneComponent.K2_GetComponentLocation` (`self.SkeletalMesh`)))
      (bind (_direction_2 _alpha_2) (`Timeline|Timeline_1` :!via `PlayFromStart`)
        (:`Update`
          (bind (_returnvalue_x_3 _returnvalue_y_3 _returnvalue_z_2) (`KismetMathLibrary.BreakVector` (`KismetMathLibrary.VLerp` (`self.GrabLocation`) (`SceneComponent.GetSocketLocation` (`Character.Mesh` (`self.boss`)) "JNT_Wrist_R_01Socket") _alpha_2)))
          (`SceneComponent.K2_SetWorldLocation` (`self.SkeletalMesh`) (`KismetMathLibrary.MakeVector` _returnvalue_x_3 _returnvalue_y_3 _returnvalue_z_2) false false)
          (if (not (`self.StopPlayerLocation`))
            (`self.K2_SetActorLocation` _returnvalue (`KismetMathLibrary.MakeVector` _returnvalue_x_2 _returnvalue_y_2 _returnvalue_z) false false)))
        (:`Finished`
          (set `self.StopPlayerLocation` false)
          (`SceneComponent.K2_AttachToComponent` (`self.SkeletalMesh`) (`self.Scene`) "None" "KeepRelative" "KeepRelative" "KeepRelative" true)
          (`SceneComponent.K2_SetRelativeTransform` (`self.SkeletalMesh`) (`KismetMathLibrary.MakeTransform` (0.0 0.0 0.0)) false false))
        (:`StopPlayerLocation`
          (`/Game/Prog/topDownBear/Blueprints/TopDownCharacter.CanMove` (cast `/Game/Prog/topDownBear/Blueprints/TopDownCharacter` (`GameplayStatics.GetPlayerCharacter` 0) :!pure true) true true)
          (set `self.StopPlayerLocation` true))))))

(event `self.ReceiveTick`
  (params (DeltaSeconds :type "Float (single-precision)")))

(event `self.SkeletalMesh.OnComponentBeginOverlap`
  (params (OverlappedComponent :type "PrimitiveComponent Object Reference") (OtherActor :type "Actor Object Reference") (OtherComp :type "PrimitiveComponent Object Reference") (OtherBodyIndex :type Integer) (bFromSweep :type Boolean) (SweepResult :type "HitResult Structure (by ref)"))
  ;[1 1 1] NOT USED
)

(event `GoBackToBoss`
  ;[1 1 1] NOT USED
)

(fn `UserConstructionScript`)