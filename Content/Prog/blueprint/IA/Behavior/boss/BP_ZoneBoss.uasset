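; Boss arena zone that stages the player's entry into and exit from a boss fight.
; BoxStart runs once: it locks input, raises entrance spikes, walks the player in while timelines blend the camera to arena settings, then starts BossRef's fight and Wwise music.
; SpikesDown lowers entrance and exit spikes once all four are valid.
; BoxEnd disables input, sends the player to MoveToEnd and blends the camera back to defaults.
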(event `self.BoxStart.OnComponentBeginOverlap`
  (params (OverlappedComponent :type "PrimitiveComponent Object Reference") (OtherActor :type "Actor Object Reference") (OtherComp :type "PrimitiveComponent Object Reference") (OtherBodyIndex :type Integer) (bFromSweep :type Boolean) (SweepResult :type "HitResult Structure (by ref)"))
  (bind _picsentree2 (`self.PicsEntree2`))
  (bind (_settings_armlength _settings_armrotation _settings_camerarotation) (break `/Game/Prog/blueprint/Camera/SpringArm_Camera_Settings` (`self.Settings`)))
  (bind (_defaultplayersettings_armlength _defaultplayersettings_armrotation _defaultplayersettings_camerarotation) (break `/Game/Prog/blueprint/Camera/SpringArm_Camera_Settings` (`self.DefaultPlayerSettings`)))
  (bind _picsentree1 (`self.PicsEntree1`))
  (bind (_returnvalue_x _returnvalue_y) (`KismetMathLibrary.BreakVector` (`self.K2_GetActorLocation` _picsentree1)))
  (bind (_returnvalue_x_2 _returnvalue_y_2) (`KismetMathLibrary.BreakVector` (`self.K2_GetActorLocation` _picsentree2)))
  (bind _roll (.roll _defaultplayersettings_armrotation))
  (bind _pitch (.pitch _defaultplayersettings_armrotation))
  (bind _yaw (.yaw _defaultplayersettings_armrotation))
  (bind _roll_2 (.roll _defaultplayersettings_camerarotation))
  (bind _pitch_2 (.pitch _defaultplayersettings_camerarotation))
  (bind _yaw_2 (.yaw _defaultplayersettings_camerarotation))
  (bind _astop_down_character (cast `/Game/Prog/topDownBear/Blueprints/TopDownCharacter` OtherActor))
  (`/Engine/EditorBlueprintResources/StandardMacros.DoOnce` false
    (:`Completed`
      (`self.DisableInput` _astop_down_character null)
      (set `/Game/Prog/topDownBear/Blueprints/TopDownCharacter.Firing?` false _astop_down_character)
      (set `/Game/Prog/topDownBear/Blueprints/TopDownCharacter.addScreen` true _astop_down_character)
      (`AkGameplayStatics.PostEvent` "/Game/sound_design/Wwise/Environment/Stop_KAli_whisper_02.Stop_KAli_whisper_02" _astop_down_character)
      (`self.CheckSpikes`
        (:`Is Valid`
          (`AkGameplayStatics.PostEvent` "/Game/sound_design/Wwise/Environment/SpikeDoor/E_SpikeDoor_Begin.E_SpikeDoor_Begin" _astop_down_character)
          (bind (_direction _alpha) (`Timeline|PicsUp` :!via `PlayFromStart`)
            (:`Update`
              (`self.K2_SetActorLocation` _picsentree1 (`KismetMathLibrary.MakeVector` _returnvalue_x _returnvalue_y _alpha) false false)
              (`self.K2_SetActorLocation` _picsentree2 (`KismetMathLibrary.MakeVector` _returnvalue_x_2 _returnvalue_y_2 _alpha) false false))
            (:`Finished`
              (`AkGameplayStatics.PostEvent` "/Game/sound_design/Wwise/Environment/SpikeDoor/E_SpikeDoor_End.E_SpikeDoor_End" _astop_down_character)
              (`|ExecutionSequence`
                (:`then_0`
                  (bind (_direction_2 _alpha_2) (`Timeline|Timeline_0`)
                    (:`Update`
                      (bind _springarm (`/Game/Prog/topDownBear/Blueprints/TopDownCharacter.SpringArm` _astop_down_character))
                      (set `SpringArmComponent.TargetArmLength` (+ (/ (* (- _settings_armlength _defaultplayersettings_armlength) _alpha_2) 100.0) _defaultplayersettings_armlength) _springarm)
                      (`SceneComponent.K2_SetRelativeRotation` _springarm (`KismetMathLibrary.MakeRotator` (+ (/ (* (- (.roll _settings_armrotation) _roll) _alpha_2) 100.0) _roll) (+ (/ (* (- (.pitch _settings_armrotation) _pitch) _alpha_2) 100.0) _pitch) (+ (/ (* (- (.yaw _settings_armrotation) _yaw) _alpha_2) 100.0) _yaw)) false false)
                      (`SceneComponent.K2_SetRelativeRotation` (`/Game/Prog/topDownBear/Blueprints/TopDownCharacter.Camera` _astop_down_character) (`KismetMathLibrary.MakeRotator` (+ (/ (* (- (.roll _settings_camerarotation) _roll_2) _alpha_2) 100.0) _roll_2) (+ (/ (* (- (.pitch _settings_camerarotation) _pitch_2) _alpha_2) 100.0) _pitch_2) (+ (/ (* (- (.yaw _settings_camerarotation) _yaw_2) _alpha_2) 100.0) _yaw_2)) false false))
                    (:`Finished`
                      (set `/Game/Prog/topDownBear/Blueprints/TopDownCharacter.BossFight` true _astop_down_character)
                      (`/Game/Prog/blueprint/IA/IA_Boss.StartFight` (`self.boss_ref`) _astop_down_character)
                      (`KismetSystemLibrary.Delay` 6.1)
                      (`self.EnableInput` _astop_down_character (`GameplayStatics.GetPlayerController` 0))
                      (set `/Game/Prog/topDownBear/Blueprints/TopDownCharacter.addScreen` false _astop_down_character)
                      (`AkGameplayStatics.SetState` "Music_Kali_STATE" "Kali_Phase1"))))
                (:`then_1`
                  (`AIBlueprintHelperLibrary.SimpleMoveToLocation` (`Pawn.GetController` _astop_down_character) (`SceneComponent.K2_GetComponentLocation` (`self.Move ToStart`))))))))))))

(event `SpikesDown`
  (bind _picsentree1 (`self.PicsEntree1`))
  (bind _picsentree2 (`self.PicsEntree2`))
  (bind _picssortie1 (`self.PicsSortie1`))
  (bind _picssortie2 (`self.PicsSortie2`))
  (bind (_returnvalue_x _returnvalue_y) (`KismetMathLibrary.BreakVector` (`self.K2_GetActorLocation` _picssortie2)))
  (bind (_returnvalue_x_2 _returnvalue_y_2) (`KismetMathLibrary.BreakVector` (`self.K2_GetActorLocation` _picsentree1)))
  (bind (_returnvalue_x_3 _returnvalue_y_3) (`KismetMathLibrary.BreakVector` (`self.K2_GetActorLocation` _picsentree2)))
  (bind (_returnvalue_x_4 _returnvalue_y_4) (`KismetMathLibrary.BreakVector` (`self.K2_GetActorLocation` _picssortie1)))
  (bind _astop_down_character (cast `/Game/Prog/topDownBear/Blueprints/TopDownCharacter` (`GameplayStatics.GetPlayerPawn` 0) :!pure true))
  (`self.CheckSpikes`
    (:`Is Valid`
      (`AkGameplayStatics.PostEvent` "/Game/sound_design/Wwise/Environment/SpikeDoor/E_SpikeDoor_Begin.E_SpikeDoor_Begin" _astop_down_character)
      (bind (_direction _alpha) (`Timeline|Timeline_1` :!via `ReverseFromEnd`)
        (:`Update`
          (`self.K2_SetActorLocation` _picsentree1 (`KismetMathLibrary.MakeVector` _returnvalue_x_2 _returnvalue_y_2 _alpha) false false)
          (`self.K2_SetActorLocation` _picsentree2 (`KismetMathLibrary.MakeVector` _returnvalue_x_3 _returnvalue_y_3 _alpha) false false)
          (`self.K2_SetActorLocation` _picssortie1 (`KismetMathLibrary.MakeVector` _returnvalue_x_4 _returnvalue_y_4 _alpha) false false)
          (`self.K2_SetActorLocation` _picssortie2 (`KismetMathLibrary.MakeVector` _returnvalue_x _returnvalue_y _alpha) false false))
        (:`Finished`
          (`AkGameplayStatics.PostEvent` "/Game/sound_design/Wwise/Environment/SpikeDoor/E_SpikeDoor_End.E_SpikeDoor_End" _astop_down_character))))))

(event `self.BoxEnd.OnComponentBeginOverlap`
  (params (OverlappedComponent :type "PrimitiveComponent Object Reference") (OtherActor :type "Actor Object Reference") (OtherComp :type "PrimitiveComponent Object Reference") (OtherBodyIndex :type Integer) (bFromSweep :type Boolean) (SweepResult :type "HitResult Structure (by ref)"))
  (bind (_defaultplayersettings_armlength _defaultplayersettings_armrotation _defaultplayersettings_camerarotation) (break `/Game/Prog/blueprint/Camera/SpringArm_Camera_Settings` (`self.DefaultPlayerSettings`)))
  (bind (_settings_armlength _settings_armrotation _settings_camerarotation) (break `/Game/Prog/blueprint/Camera/SpringArm_Camera_Settings` (`self.Settings`)))
  (bind _roll (.roll _settings_armrotation))
  (bind _pitch (.pitch _settings_armrotation))
  (bind _yaw (.yaw _settings_armrotation))
  (bind _roll_2 (.roll _settings_camerarotation))
  (bind _pitch_2 (.pitch _settings_camerarotation))
  (bind _yaw_2 (.yaw _settings_camerarotation))
  (bind _astop_down_character (cast `/Game/Prog/topDownBear/Blueprints/TopDownCharacter` OtherActor))
  (set `/Game/Prog/topDownBear/Blueprints/TopDownCharacter.addScreen` true _astop_down_character)
  (`self.DisableInput` _astop_down_character null)
  (set `/Game/Prog/topDownBear/Blueprints/TopDownCharacter.Firing?` false _astop_down_character)
  (set `CharacterMovementComponent.MaxWalkSpeed` 200.0 (`Character.CharacterMovement` _astop_down_character))
  (set `/Game/Prog/topDownBear/Blueprints/TopDownCharacter.MoveTo?` true _astop_down_character)
  (set `/Game/Prog/topDownBear/Blueprints/TopDownCharacter.locMoveTo` (`SceneComponent.K2_GetComponentLocation` (`self.MoveToEnd`)) _astop_down_character)
  (bind (_direction _alpha) (`Timeline|Timeline_2`)
    (:`Update`
      (bind _springarm (`/Game/Prog/topDownBear/Blueprints/TopDownCharacter.SpringArm` _astop_down_character))
      (set `SpringArmComponent.TargetArmLength` (+ (/ (* (- _defaultplayersettings_armlength _settings_armlength) _alpha) 100.0) _settings_armlength) _springarm)
      (`SceneComponent.K2_SetRelativeRotation` _springarm (`KismetMathLibrary.MakeRotator` (+ (/ (* (- (.roll _defaultplayersettings_armrotation) _roll) _alpha) 100.0) _roll) (+ (/ (* (- (.pitch _defaultplayersettings_armrotation) _pitch) _alpha) 100.0) _pitch) (+ (/ (* (- (.yaw _defaultplayersettings_armrotation) _yaw) _alpha) 100.0) _yaw)) false false)
      (`SceneComponent.K2_SetRelativeRotation` (`/Game/Prog/topDownBear/Blueprints/TopDownCharacter.Camera` _astop_down_character) (`KismetMathLibrary.MakeRotator` (+ (/ (* (- (.roll _defaultplayersettings_camerarotation) _roll_2) _alpha) 100.0) _roll_2) (+ (/ (* (- (.pitch _defaultplayersettings_camerarotation) _pitch_2) _alpha) 100.0) _pitch_2) (+ (/ (* (- (.yaw _defaultplayersettings_camerarotation) _yaw_2) _alpha) 100.0) _yaw_2)) false false))))

(fn `UserConstructionScript`)