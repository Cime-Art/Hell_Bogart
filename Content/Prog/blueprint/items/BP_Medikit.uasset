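; BP_Medikit is a health kit pickup that adds one medikit to the player's TopDownCharacter on overlap.
; The overlap event casts to the character, increments its Medikit count, posts the Wwise pickup sound, sets Finished, calls UpdateGameInstance and destroys itself.
; An AlreadyFinished event prints a debug string and destroys the actor, apparently for kits already collected.
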(event `self.Medikit.OnComponentBeginOverlap`
  (params (OverlappedComponent :type "PrimitiveComponent Object Reference") (OtherActor :type "Actor Object Reference") (OtherComp :type "PrimitiveComponent Object Reference") (OtherBodyIndex :type Integer) (bFromSweep :type Boolean) (SweepResult :type "HitResult Structure (by ref)"))
  (bind _astop_down_character (cast `/Game/Prog/topDownBear/Blueprints/TopDownCharacter` OtherActor))
  (`/Engine/EditorBlueprintResources/StandardMacros.IncrementInt` (`/Game/Prog/topDownBear/Blueprints/TopDownCharacter.medikit` _astop_down_character)
    (:`  `
      (`AkGameplayStatics.PostEvent` "/Game/sound_design/Wwise/PickUp/HB_PickUpHealthkit.HB_PickUpHealthkit" self)
      (set `self.?Finished` true)
      (`self.UpdateGameInstance`)
      (`self.K2_DestroyActor`))))

(event `self.AlreadyFinished`
  (`KismetSystemLibrary.PrintString` "AlreadyFinished")
  (`self.K2_DestroyActor`))

(fn `UserConstructionScript`)