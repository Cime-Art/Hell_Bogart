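; BP_Item is a physical item actor whose look and stats come from the ItemsBase data table.
; Creation looks up the row named by ItemName, stores its mesh, material, name, value and rarity, then passes them to Initialization.
; Initialization applies the mesh and material at half scale, enables physics and launches the item away from the player cached at BeginPlay with an impulse.
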(event `self.ReceiveBeginPlay`
  (set `self.player` (`GameplayStatics.GetPlayerCharacter` 0)))

(fn `creation`
  (bind _returnvalue (`|GetDataTableRow` "/Game/Prog/dataBase/item/itemsBase.itemsBase" (`self.itemName`))
    (:`then`
      (bind (_index _itemmesh _itemmat _itemname _itemvalue _rarity) (break `/Game/Prog/dataBase/item/itemsStructure` _returnvalue))
      (set `self.itemMesh` _itemmesh)
      (set `self.itemMat` _itemmat)
      (set `self.itemName` _itemname)
      (set `self.itemValue` _itemvalue)
      (set `self.itemRarity` _rarity)
      (`self.initialization` _itemmesh _itemmat _itemname _itemvalue _rarity))))

(fn `initialization`
  (params (itemMesh :type "StaticMesh Object Reference") (itemMat :type "Material Object Reference") (itemName :type Name) (itemValue :type "Map of Name to Float (double-precision)") (itemRarity :type Integer))
  (bind _staticmesh (`self.StaticMesh`))
  (`StaticMeshComponent.SetStaticMesh` _staticmesh itemMesh)
  (`PrimitiveComponent.SetSimulatePhysics` _staticmesh true)
  (`SceneComponent.SetWorldScale3D` _staticmesh (0.5 0.5 0.5))
  (`PrimitiveComponent.SetMaterial` _staticmesh 0 itemMat)
  (`PrimitiveComponent.AddImpulse` _staticmesh (* (`KismetMathLibrary.GetDirectionUnitVector` (`self.K2_GetActorLocation` (`self.player`)) (`self.K2_GetActorLocation`)) 50000.0) "None" false))

(fn `UserConstructionScript`)