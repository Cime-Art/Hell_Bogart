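; One-shot trigger door for Zone C that swings two stone leaves open and can end the game on the credits screen.
; The first TopDownCharacter overlap starts a timeline rotating the leaves in opposite yaw directions from their starting angles, with Niagara effects and Wwise audio.
; A second timeline then drives the character's screen opacity.
; When it finishes on map Zone_Tampon_C, the Credit widget appears and the game pauses.
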(event `self.ReceiveBeginPlay`
  (bind (_returnvalue_roll _returnvalue_pitch _returnvalue_yaw) (`KismetMathLibrary.BreakRotator` (`SceneComponent.K2_GetComponentRotation` (`self.porte_droite`))))
  (bind (_returnvalue_roll_2 _returnvalue_pitch_2 _returnvalue_yaw_2) (`KismetMathLibrary.BreakRotator` (`SceneComponent.K2_GetComponentRotation` (`self.porte_gauche`))))
  (set `self.originalYaw_PorteDroite` _returnvalue_yaw)
  (set `self.originalYaw_PorteGauche` _returnvalue_yaw_2))

(event `self.BoxDoor.OnComponentBeginOverlap`
  (params (OverlappedComponent :type "PrimitiveComponent Object Reference") (OtherActor :type "Actor Object Reference") (OtherComp :type "PrimitiveComponent Object Reference") (OtherBodyIndex :type Integer) (bFromSweep :type Boolean) (SweepResult :type "HitResult Structure (by ref)"))
  (bind _originalyaw_portedroite (`self.originalYaw_PorteDroite`))
  (bind _originalyaw_portegauche (`self.originalYaw_PorteGauche`))
  (bind _astop_down_character (cast `/Game/Prog/topDownBear/Blueprints/TopDownCharacter` OtherActor))
  (`/Engine/EditorBlueprintResources/StandardMacros.DoOnce` false
    (:`Completed`
      (`|ExecutionSequence`
        (:`then_0`
          (`AkGameplayStatics.PostEvent` "/Game/sound_design/Wwise/Global/E_Enable_Attenuation.E_Enable_Attenuation" self)
          (`AkGameplayStatics.PostEvent` "/Game/sound_design/Wwise/Environment/BigStoneDoor/E_BigStoneDoor_Opening.E_BigStoneDoor_Opening" self)
          (`ActorComponent.Activate` (`self.Niagara`) false)
          (`ActorComponent.Activate` (`self.Niagara1`) false)
          (bind (_direction _alpha) (`Timeline|OpenDoors`)
            (:`Update`
              (`SceneComponent.K2_SetWorldRotation` (`self.porte_droite`) (`KismetMathLibrary.MakeRotator` 0.0 0.0 (`KismetMathLibrary.MapRangeClamped` _alpha 0.0 1.0 _originalyaw_portedroite (+ _originalyaw_portedroite 60.0))) false false)
              (`SceneComponent.K2_SetWorldRotation` (`self.porte_gauche`) (`KismetMathLibrary.MakeRotator` 0.0 0.0 (`KismetMathLibrary.MapRangeClamped` _alpha 0.0 1.0 _originalyaw_portegauche (- _originalyaw_portegauche 60.0))) false false))
            (:`Finished`
              (`AkGameplayStatics.PostEvent` "/Game/sound_design/Wwise/Environment/BigStoneDoor/E_BigStoneDoor_Stop.E_BigStoneDoor_Stop" self)
              (`ActorComponent.Deactivate` (`self.Niagara`))
              (`ActorComponent.Deactivate` (`self.Niagara1`))
              (bind (_direction_2 _newtrack_0) (`Timeline|Timeline_0`)
                (:`Update`
                  (set `/Game/Prog/topDownBear/Blueprints/TopDownCharacter.opacityScreen` _newtrack_0 _astop_down_character))
                (:`Finished`
                  (if (== (`/Game/Prog/topDownBear/Blueprints/TopDownCharacter.currentMap` _astop_down_character) "Zone_Tampon_C")
                    (bind _returnvalue (`|CreateWidget` "/Game/Prog/blueprint/Widget/Credit.Credit_C"))
                    (bind _output_get (set `/Game/Prog/topDownBear/Blueprints/TopDownCharacter.parentWg` _returnvalue _astop_down_character))
                    (`UserWidget.AddToViewport` _output_get 0)
                    (`self.EnableInput` _astop_down_character (`GameplayStatics.GetPlayerController` 0))
                    (`GameplayStatics.SetGamePaused` true)))))))
        (:`then_1`
          (if (`self.zoneC`)
            _))))))

(fn `UserConstructionScript`)