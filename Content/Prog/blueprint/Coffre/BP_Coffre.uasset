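; BP_Coffre is a loot chest that shows its mesh and can open only when LoadChest is set.
; OpenChest calls Activate, which once plays the animation, hands ItemsToSpawn to ItemSpawn after a delay, and posts a Wwise music event chosen by the player's current map.
; SpawnAgain is a delayed recursive test spawner, uncalled here, that drops chance-rolled BP_Items at scattered positions and stops at the first failed roll.
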(event `SpawnAgain`
  (bind _returnvalue (`KismetMathLibrary.RandomFloatInRange` -50.0 50.0))
  (bind (_returnvalue_x _returnvalue_y _returnvalue_z) (`KismetMathLibrary.BreakVector` (`SceneComponent.K2_GetComponentLocation` (`self.locationSpawnItem`))))
  (if (`self.loadChest`)
    ;[1 1 1] Tests delay entre les spawn
    (bind _keys (`BlueprintMapLibrary.Map_Keys` (`self.itemsToSpawn`)))
    (bind _output (`|GetArrayItem` _keys (`self.dropCount`)))
    (if (<= (`KismetMathLibrary.RandomFloat`) (`BlueprintMapLibrary.Map_Find` (`self.itemsToSpawn`) _output))
      (`KismetSystemLibrary.PrintString` (`KismetStringLibrary.Conv_DoubleToString` _returnvalue))
      (bind _returnvalue_2 (`|SpawnActorFromClass` "/Game/Prog/blueprint/items/BP_Item.BP_Item_C" (`KismetMathLibrary.MakeTransform` (`KismetMathLibrary.MakeVector` (+ _returnvalue_x _returnvalue) (+ _returnvalue_y (`KismetMathLibrary.RandomFloatInRange` -50.0 50.0)) _returnvalue_z)) "AdjustIfPossibleButAlwaysSpawn" "OverrideRootScale" null null))
      (set `/Game/Prog/blueprint/items/BP_Item.itemName` _output _returnvalue_2)
      (`/Game/Prog/blueprint/items/BP_Item.creation` _returnvalue_2 0.0)
      (`/Engine/EditorBlueprintResources/StandardMacros.IncrementInt` (`self.dropCount`)
        (:`  `
          (if (< (`self.dropCount`) (`BlueprintMapLibrary.Map_Length` (`self.itemsToSpawn`)))
            (`KismetSystemLibrary.Delay` 0.2)
            (`self.SpawnAgain`)))))))

(event `self.ReceiveBeginPlay`
  (`self.chestLoad`))

(event `chestLoad`
  (bind _coffre (`self.coffre`))
  (if (`self.loadChest`)
    (`SkinnedMeshComponent.SetSkinnedAssetAndUpdate` _coffre (`self.meshChest`) true)
    (else
      (`SkinnedMeshComponent.SetSkinnedAssetAndUpdate` _coffre null true))))

(event `Activate`
  (bind _astop_down_character (cast `/Game/Prog/topDownBear/Blueprints/TopDownCharacter` (`GameplayStatics.GetPlayerPawn` 0) :!pure true))
  (bind _currentmap (`/Game/Prog/topDownBear/Blueprints/TopDownCharacter.currentMap` _astop_down_character))
  (if (`self.loadChest`)
    (`/Engine/EditorBlueprintResources/StandardMacros.DoOnce` false
      (:`Completed`
        (set `self.Open` true)
        (`|ExecutionSequence`
          (:`then_0`
            (`SkeletalMeshComponent.PlayAnimation` (`self.coffre`) (`self.animation`) false)
            (`KismetSystemLibrary.Delay` 0.5)
            (`/Game/Prog/blueprint/itemSpawn.ItemLoot` (`self.itemSpawn`) (`self.x1PerCoffre`) (`self.itemsToSpawn`) (`SceneComponent.K2_GetComponentLocation` (`self.locationSpawnItem`)) 10.0))
          (:`then_1`
            (switch `name` _currentmap
              (:`Default`
                (if (`KismetStringLibrary.Contains` (`KismetStringLibrary.Conv_NameToString` _currentmap) "2")
                  (`AkGameplayStatics.PostEvent` "/Game/sound_design/Wwise/Music/Ruins/E_Mus_Ruin_TriggerEnigmeChest.E_Mus_Ruin_TriggerEnigmeChest" _astop_down_character)
                  (else
                    (`AkGameplayStatics.PostEvent` "/Game/sound_design/Wwise/Music/Jungle/E_Mus_TriggerEnigmeChest.E_Mus_TriggerEnigmeChest" _astop_down_character)))))))))))

(event `OpenChest`
  (`self.Activate`))

(fn `UserConstructionScript`
  (bind _mesh (`self.mesh`))
  (`SkinnedMeshComponent.SetSkinnedAssetAndUpdate` (`self.coffre`) _mesh true)
  (set `self.meshChest` _mesh))