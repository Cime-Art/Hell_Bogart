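; SlowArea is a grenade-related area effect that slows enemies inside it for a limited time.
; On begin play it scales its Sphere into a wide, flatter volume.
; Sphere overlaps set each BP_Ennemy's Slowed flag and call its Slow function, clearing it when the enemy leaves.
; Tick accumulates a timer and destroys the actor once TimerLifeTime is reached.
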(event `self.ReceiveBeginPlay`
  (`SceneComponent.SetWorldScale3D` (`self.Sphere`) (3.0 3.0 1.0)))

(event `self.ReceiveTick`
  (params (DeltaSeconds :type "Float (single-precision)"))
  (bind _output_get (set `self.timer` (+ DeltaSeconds (`self.timer`))))
  (if (>= _output_get (`self.timerLifeTime`))
    (`self.K2_DestroyActor`)))

(event `self.Sphere.OnComponentBeginOverlap`
  (params (OverlappedComponent :type "PrimitiveComponent Object Reference") (OtherActor :type "Actor Object Reference") (OtherComp :type "PrimitiveComponent Object Reference") (OtherBodyIndex :type Integer) (bFromSweep :type Boolean) (SweepResult :type "HitResult Structure (by ref)"))
  (bind _asbp_ennemy (cast `/Game/Prog/blueprint/IA/BP_Ennemy` OtherActor))
  (bind _output_get (set `/Game/Prog/blueprint/IA/BP_Ennemy.slowed` true _asbp_ennemy))
  (`/Game/Prog/blueprint/IA/BP_Ennemy.slow` _asbp_ennemy _output_get))

(event `self.Sphere.OnComponentEndOverlap`
  (params (OverlappedComponent :type "PrimitiveComponent Object Reference") (OtherActor :type "Actor Object Reference") (OtherComp :type "PrimitiveComponent Object Reference") (OtherBodyIndex :type Integer))
  (bind _asbp_ennemy (cast `/Game/Prog/blueprint/IA/BP_Ennemy` OtherActor))
  (bind _output_get (set `/Game/Prog/blueprint/IA/BP_Ennemy.slowed` false _asbp_ennemy))
  (`/Game/Prog/blueprint/IA/BP_Ennemy.slow` _asbp_ennemy _output_get))

(fn `UserConstructionScript`)