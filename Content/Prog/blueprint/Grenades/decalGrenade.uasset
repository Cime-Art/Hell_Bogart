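; Grenade decal Blueprint that leaves fading ice, fire or thunder marks on the ground.
; IsGround traces 100 units down and stores the impact point as the decal location.
; Each element event spawns a decal with a dynamic material, plays its own Timeline to drive Opacity, then destroys the decal.
; Ice and fire decals also set EmissivePower from a three-level rarity selection; thunder does not.
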(event `decalsIce`
  (params (DecalSize :type "Vector Structure") (Selection :type String))
  (bind _materialice (`self.materialIce`))
  (bind _returnvalue (`GameplayStatics.SpawnDecalAtLocation` "/Game/Graphs/Asset_Defs/Decals/Mat/Mat_Inst/Trace_Grenade/IceGreande_DECAL_Inst.IceGreande_DECAL_Inst" DecalSize (`self.locationGround`)))
  (bind _returnvalue_2 (`DecalComponent.CreateDynamicMaterialInstance` _returnvalue))
  (bind _output_get (set `self.materialIce` _returnvalue_2))
  (`DecalComponent.SetDecalMaterial` _returnvalue _output_get)
  (`self.raretydecals` Selection _materialice)
  (bind (_direction _opacity) (`Timeline|Timeline_0` :!via `PlayFromStart`)
    (:`Update`
      (`MaterialInstanceDynamic.SetScalarParameterValue` _materialice "Opacity" _opacity))
    (:`Finished`
      (`ActorComponent.K2_DestroyComponent` _returnvalue))))

(event `FireDecals`
  (params (DecalSize :type "Vector Structure") (NewParam :type String))
  (bind _returnvalue (`GameplayStatics.SpawnDecalAtLocation` "/Game/Graphs/Asset_Defs/Decals/Mat/Mat_Inst/Trace_Grenade/FlameGreande_DECAL_Inst.FlameGreande_DECAL_Inst" DecalSize (`self.locationGround`)))
  (bind _returnvalue_2 (`DecalComponent.CreateDynamicMaterialInstance` _returnvalue))
  (bind _output_get (set `self.matFire` _returnvalue_2))
  (`DecalComponent.SetDecalMaterial` _returnvalue _output_get)
  (`self.raretydecals` NewParam (`self.matFire`))
  (bind (_direction _opacity) (`Timeline|Timeline_1` :!via `PlayFromStart`)
    (:`Update`
      (`MaterialInstanceDynamic.SetScalarParameterValue` (`self.matFire`) "Opacity" _opacity))
    (:`Finished`
      (`ActorComponent.K2_DestroyComponent` _returnvalue))))

(event `ThunderDecals`
  (params (DecalSize :type "Vector Structure"))
  (bind _returnvalue (`GameplayStatics.SpawnDecalAtLocation` "/Game/Graphs/Asset_Defs/Decals/Mat/Mat_Inst/Trace_Grenade/M_Trace_Grenade_Inst.M_Trace_Grenade_Inst" DecalSize (`self.locationGround`)))
  (bind _returnvalue_2 (`DecalComponent.CreateDynamicMaterialInstance` _returnvalue))
  (bind _output_get (set `self.thunderMat` _returnvalue_2))
  (`DecalComponent.SetDecalMaterial` _returnvalue _output_get)
  (bind (_direction _opacity) (`Timeline|Timeline_2` :!via `PlayFromStart`)
    (:`Update`
      (`MaterialInstanceDynamic.SetScalarParameterValue` (`self.thunderMat`) "Opacity" _opacity))
    (:`Finished`
      (`ActorComponent.K2_DestroyComponent` _returnvalue))))

(fn `isGround`
  (params (actorLocation :type "Vector Structure"))
  (returns (ReturnValue :type Boolean))
  (bind (_outhit _returnvalue) (`KismetSystemLibrary.LineTraceSingleForObjects` actorLocation (- actorLocation (0.0 0.0 100.0)) (`|MakeArray` "ObjectTypeQuery7" :!type "EObjectTypeQuery Enum")))
  (set `self.locationGround` (`.ImpactPoint` (`GameplayStatics.BreakHitResult` _outhit)))
  (return _returnvalue))

(fn `raretydecals`
  (params (Selection :type String) (Target :type "MaterialInstanceDynamic Object Reference"))
  (switch `string` Selection
    (:`1`
      (`MaterialInstanceDynamic.SetScalarParameterValue` Target "EmissivePower" 20.0))
    (:`2`
      (`MaterialInstanceDynamic.SetScalarParameterValue` Target "EmissivePower" 80.0))
    (:`3`
      (`MaterialInstanceDynamic.SetScalarParameterValue` Target "EmissivePower" 150.0))))

(fn `UserConstructionScript`)