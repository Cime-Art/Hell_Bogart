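; Ice grenade Blueprint that freezes enemies overlapping its explosion radius, extending a parent grenade's explosion logic.
; On explosion, it spawns a decal actor and checks for ground, placing a rarity-scaled ice effect and decal there, or an in-air effect otherwise.
; Radius overlaps call TurnFreezed on BP_Enemy actors, with a freeze time selected from the grenade's three rarity tiers.
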(event `self.Grenade explosion`
  (`parent.Grenade explosion`)
  (bind _returnvalue (`|SpawnActorFromClass` "/Game/Prog/blueprint/Grenades/decalGrenade.decalGrenade_C" (`self.GetTransform`) "Undefined" "OverrideRootScale" null null))
  (set `self.iceDecal` _returnvalue)
  (bind _returnvalue_2 (`/Game/Prog/blueprint/Grenades/decalGrenade.isGround` (`self.iceDecal`) (`self.K2_GetActorLocation`)))
  (if _returnvalue_2
    (switch `string` (`self.rarity`)
      (:`1`
        (`GameplayStatics.SpawnEmitterAtLocation` "/Game/Graphs/Particles/Grenade/Ice_Grenade/G-Ice_S.G-Ice_S" (`self.K2_GetActorLocation`) (struct) (1.5 1.5 1.5))
        (`/Game/Prog/blueprint/Grenades/decalGrenade.decalsIce` (`self.iceDecal`) (90.0 180.0 180.0) (`self.rarity`)))
      (:`2`
        (`GameplayStatics.SpawnEmitterAtLocation` "/Game/Graphs/Particles/Grenade/Ice_Grenade/G-Ice_R.G-Ice_R" (`self.K2_GetActorLocation`) (struct) (1.5 1.5 1.5))
        (`/Game/Prog/blueprint/Grenades/decalGrenade.decalsIce` (`self.iceDecal`) (128.0 256.0 256.0) (`self.rarity`)))
      (:`3`
        (`GameplayStatics.SpawnEmitterAtLocation` "/Game/Graphs/Particles/Grenade/Ice_Grenade/G-Ice_L.G-Ice_L" (`self.K2_GetActorLocation`) (struct) (2.0 2.0 2.0))
        (`/Game/Prog/blueprint/Grenades/decalGrenade.decalsIce` (`self.iceDecal`) (200.0 400.0 400.0) (`self.rarity`))))
    (else
      (`GameplayStatics.SpawnEmitterAtLocation` "/Game/Graphs/Particles/Grenade/Ice_Grenade/G-Ice_InAir.G-Ice_InAir" (`self.K2_GetActorLocation`)))))

(event `self.radius explo.OnComponentBeginOverlap`
  (params (OverlappedComponent :type "PrimitiveComponent Object Reference") (OtherActor :type "Actor Object Reference") (OtherComp :type "PrimitiveComponent Object Reference") (OtherBodyIndex :type Integer) (bFromSweep :type Boolean) (SweepResult :type "HitResult Structure (by ref)"))
  (bind _asbp_enemy (cast `/Game/Prog/blueprint/IA/BP_Enemy` OtherActor))
  (switch `string` (`self.rarity`)
    (:`1`
      (set `self.timeFreeze` (`self.timeFreezeStandard`)))
    (:`2`
      (set `self.timeFreeze` (`self.timeFreezeRare`)))
    (:`3`
      (set `self.timeFreeze` (`self.timeFreezeLegendaire`))))
  (`/Game/Prog/blueprint/IA/BP_Enemy.TurnFreezed` _asbp_enemy (`self.timeFreeze`)))

(fn `UserConstructionScript`
  (`parent.UserConstructionScript`))