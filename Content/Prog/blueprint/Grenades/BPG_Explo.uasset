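; Grenade Blueprint, a child class, that explodes on a timer.
; Tick accumulates delta time until it reaches TimeBeforeExplosion, then a DoOnce gate fires GrenadeExplosion once with the EmitterExplosion effect.
; The construction script only calls its parent.
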(event `self.ReceiveTick`
  (params (DeltaSeconds :type "Float (single-precision)"))
  (bind _output_get (set `self.timer` (+ DeltaSeconds (`self.timer`))))
  (if (>= _output_get (`self.timeBeforeExplosion`))
    (`/Engine/EditorBlueprintResources/StandardMacros.DoOnce` false
      (:`Completed`
        (`self.Grenade explosion` (`self.EmitterExplosion`))))))

(fn `UserConstructionScript`
  (`parent.UserConstructionScript`))