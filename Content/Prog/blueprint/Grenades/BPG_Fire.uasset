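; Fire grenade Blueprint that explodes on a timer and sets enemies alight.
; Tick accumulates elapsed time and calls GrenadeExplosion once, through a DoOnce, when TimeBeforeExplosion is reached.
; Any BP_Ennemy that begins overlapping the RadiusExplo component receives the FireDmg value and has Burning set to true.
; The construction script only calls its parent.
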(event `self.ReceiveTick`
  (params (DeltaSeconds :type "Float (single-precision)"))
  (bind _output_get (set `self.timer` (+ DeltaSeconds (`self.timer`))))
  (if (>= _output_get (`self.timeBeforeExplosion`))
    (`/Engine/EditorBlueprintResources/StandardMacros.DoOnce` false
      (:`Completed`
        (`self.Grenade explosion`)))))

(event `self.radius explo.OnComponentBeginOverlap`
  (params (OverlappedComponent :type "PrimitiveComponent Object Reference") (OtherActor :type "Actor Object Reference") (OtherComp :type "PrimitiveComponent Object Reference") (OtherBodyIndex :type Integer) (bFromSweep :type Boolean) (SweepResult :type "HitResult Structure (by ref)"))
  (bind _asbp_ennemy (cast `/Game/Prog/blueprint/IA/BP_Ennemy` OtherActor))
  (set `/Game/Prog/blueprint/IA/BP_Ennemy.FireDmg` (`self.fireDmg`) _asbp_ennemy)
  (set `/Game/Prog/blueprint/IA/BP_Ennemy.burning` true _asbp_ennemy))

(fn `UserConstructionScript`
  (`parent.UserConstructionScript`))