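; Lightning grenade that shocks and slows enemies, extending a parent grenade's explosion logic.
; On explosion it spawns a decal actor to test for ground, then plays either a rarity-based effect with a sized thunder decal or a mid-air effect.
; Enemies beginning overlap with the explosion radius receive a Thunder call, with tick count, electric damage and slow time all scaled by rarity.
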(event `self.Grenade explosion`
  (bind _returnvalue (- (`self.rarity`) 1))
  (`parent.Grenade explosion`)
  (bind _returnvalue_2 (`|SpawnActorFromClass` "/Game/Prog/blueprint/Grenades/decalGrenade.decalGrenade_C" (`self.GetTransform`) "Undefined" "OverrideRootScale" null null))
  (set `self.thunderDecal` _returnvalue_2)
  (bind _returnvalue_3 (`/Game/Prog/blueprint/Grenades/decalGrenade.isGround` (`self.thunderDecal`) (`self.K2_GetActorLocation`)))
  (if _returnvalue_3
    (`GameplayStatics.SpawnEmitterAtLocation` (select `int` _returnvalue :`0` "/Game/Graphs/Particles/Grenade/Electric_Grenade/Grenade_E_Standard.Grenade_E_Standard" :`1` "/Game/Graphs/Particles/Grenade/Electric_Grenade/Grenade_E_Rare.Grenade_E_Rare" :`2` "/Game/Graphs/Particles/Grenade/Electric_Grenade/Grenade_E_Epique.Grenade_E_Epique" :!type "ParticleSystem Object Reference") (`self.K2_GetActorLocation`) (struct) (1.5 1.5 1.5))
    (`/Game/Prog/blueprint/Grenades/decalGrenade.ThunderDecals` (`self.thunderDecal`) (select `int` _returnvalue :`0` (90.0 180.0 180.0) :`1` (128.0 256.0 256.0) :`2` (200.0 400.0 400.0) :!type "Vector Structure"))
    (else
      (`GameplayStatics.SpawnEmitterAtLocation` "/Game/Graphs/Particles/Grenade/Electric_Grenade/Grenade_E_InAir.Grenade_E_InAir" (`self.K2_GetActorLocation`)))))

(event `self.radius explo.OnComponentBeginOverlap`
  (params (OverlappedComponent :type "PrimitiveComponent Object Reference") (OtherActor :type "Actor Object Reference") (OtherComp :type "PrimitiveComponent Object Reference") (OtherBodyIndex :type Integer) (bFromSweep :type Boolean) (SweepResult :type "HitResult Structure (by ref)"))
  (bind _returnvalue (select `int` (- (`self.rarity`) 1) :`0` 5.0 :`1` 10.0 :`2` 15.0))
  (bind _asbp_enemy (cast `/Game/Prog/blueprint/IA/BP_Enemy` OtherActor))
  (`/Game/Prog/blueprint/IA/BP_Enemy.Thunder` _asbp_enemy (`KismetMathLibrary.FTrunc` _returnvalue) (`KismetMathLibrary.FTrunc` (select `int` (- (`self.rarity`) 1) :`0` 50.0 :`1` 100.0 :`2` 150.0)) _returnvalue))

(fn `UserConstructionScript`
  (`parent.UserConstructionScript`))