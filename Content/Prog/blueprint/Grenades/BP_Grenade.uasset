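; BP_Grenade is a grenade actor that explodes on demand and damages nearby enemies.
; Its Grenadeexplosion event enables and resizes an overlap sphere to the blast radius, spawns a given particle effect, plays a Wwise sound, then destroys the actor.
; Enemies entering the sphere during that resize receive GetDamage with damage, a grenade reference and explosion force.
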(event `Grenade explosion`
  (params (EmitterTemplate :type "ParticleSystem Object Reference"))
  (`PrimitiveComponent.SetCollisionProfileName` (`self.radius explo`) "OverlapAllDynamic")
  (`SphereComponent.SetSphereRadius` (`self.radius explo`) (`self.radiusExplo`) true)
  (`GameplayStatics.SpawnEmitterAtLocation` EmitterTemplate (`self.K2_GetActorLocation`) (struct :`Pitch` 90.0) (1.5 1.5 1.5))
  (`AkGameplayStatics.PostEventAtLocation` "/Game/sound_design/Wwise/Character/Grenades/E_Play_Grenade.E_Play_Grenade" (`self.K2_GetActorLocation`))
  (`self.K2_DestroyActor`))

(event `self.radius explo.OnComponentBeginOverlap`
  (params (OverlappedComponent :type "PrimitiveComponent Object Reference") (OtherActor :type "Actor Object Reference") (OtherComp :type "PrimitiveComponent Object Reference") (OtherBodyIndex :type Integer) (bFromSweep :type Boolean) (SweepResult :type "HitResult Structure (by ref)"))
  (bind _asbp_ennemy (cast `/Game/Prog/blueprint/IA/BP_Ennemy` OtherActor))
  (`/Game/Prog/blueprint/IA/BP_Ennemy.GetDamage` _asbp_ennemy (`self.damage`) null self (`self.forceExplo`) (0.0 0.0 0.0)))

(fn `UserConstructionScript`)