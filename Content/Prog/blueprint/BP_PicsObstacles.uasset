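; Spike obstacle (Pics) that lowers out of the way once its check area holds no BP_Enemy actors.
; Every Tick polls the AreaToCheck box, and the first empty result plays the Open timeline through a DoOnce.
; The timeline moves Pics down in world Z from InitialZ.
; The construction script sizes the box from BoxExtent and caches the actor's Z as InitialZ.
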(event `self.ReceiveTick`
  (params (DeltaSeconds :type "Float (single-precision)"))
  (bind _pics (`self.Pics`))
  (bind (_returnvalue_x _returnvalue_y) (`KismetMathLibrary.BreakVector` (`SceneComponent.K2_GetComponentLocation` _pics)))
  (if (== (`KismetArrayLibrary.Array_Length` (`PrimitiveComponent.GetOverlappingActors` (`self.AreaToCheck`) "/Game/Prog/blueprint/IA/BP_Enemy.BP_Enemy_C")) 0)
    (`/Engine/EditorBlueprintResources/StandardMacros.DoOnce` false
      (:`Completed`
        (bind (_direction _value) (`Timeline|open` :!via `PlayFromStart`)
          (:`Update`
            (`SceneComponent.K2_SetWorldLocation` _pics (`KismetMathLibrary.MakeVector` _returnvalue_x _returnvalue_y (- (`self.InitialZ`) _value)) false false)))))))

(fn `UserConstructionScript`
  (bind (_returnvalue_x _returnvalue_y _returnvalue_z) (`KismetMathLibrary.BreakVector` (`self.K2_GetActorLocation`)))
  (`BoxComponent.SetBoxExtent` (`self.AreaToCheck`) (`self.boxExtent`) true)
  (set `self.InitialZ` _returnvalue_z))