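; A trigger box that plays a Wwise voice line once when the player's top-down character enters it.
; On overlap it posts the configured Ak event on the character, sets a Finished flag and calls UpdateGameInstance.
; An AlreadyFinished event sets the same flag without playing the line, so the box stays silent afterwards.
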(event `self.TriggerBox.OnComponentBeginOverlap`
  (params (OverlappedComponent :type "PrimitiveComponent Object Reference") (OtherActor :type "Actor Object Reference") (OtherComp :type "PrimitiveComponent Object Reference") (OtherBodyIndex :type Integer) (bFromSweep :type Boolean) (SweepResult :type "HitResult Structure (by ref)"))
  (if (not (`self.?Finished`))
    (bind _astop_down_character (cast `/Game/Prog/topDownBear/Blueprints/TopDownCharacter` OtherActor))
    (`AkGameplayStatics.PostEvent` (`self.AkVoiceLine`) _astop_down_character)
    (set `self.?Finished` true)
    (`self.UpdateGameInstance`)))

(event `self.AlreadyFinished`
  (set `self.?Finished` true))

(fn `UserConstructionScript`
  (`parent.UserConstructionScript`))